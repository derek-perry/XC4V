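; Shield generator whose health the player restores by drilling in the add-in area and enemies drain during waves.
; Looping-style Timelines act as ticks, polling overlaps into flags that drive health changes and player-shielded state.
; Zero health, or the player entering GeneratorCollider, plays a shutdown sound and hides the shield.
; Health and repair texts face the camera, while a dynamic glass material blends red and blue during waves.
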(event `self.ReceiveBeginPlay`
  ;[1 0 0] BeginPlay
  (`|ExecutionSequence`
    (:`then_0`
      ;[1 1 1] SavePlayer
      (bind _asxc4vcharacter (cast `/Game/XC4VCharacter/XC4VCharacter` (`GameplayStatics.GetPlayerCharacter` 0)))
      (set `self.XC4VCharacter` _asxc4vcharacter)
      ;[1 1 1] Save Generator
      (set `/Game/XC4VCharacter/XC4VCharacter.Generator` self (`self.XC4VCharacter`))
      ;[1 1 1] Create Dynamic ShieldGlass Mat
      (bind _returnvalue (`PrimitiveComponent.CreateDynamicMaterialInstance` (`self.GeneratedShieldGlass`) 0 (`PrimitiveComponent.GetMaterial` (`self.GeneratedShieldGlass`) 0) "ShieldGlassDynMat"))
      (set `self.ShieldGlassDynMaterial` _returnvalue))
    (:`then_1`
      ;[1 1 1] OverlapChecker
      (`self.CheckforOverlaps`))
    (:`then_2`
      ;[1 1 1] ShieldHealthManagement
      (`|ExecutionSequence`
        (:`then_0`
          (`self.StatusChecking`))))
    (:`then_3`
      ;[1 1 1] Health Display
      (`self.SetText`))
    (:`then_4`
      (`self.RotateTexttoPlayer`))
    (:`then_5`
      ;[1 1 1] WaveWarning
      (`self.WaveWarning`))))

(event `CheckforOverlaps`
  (bind _shieldhealthrepairtext (`self.ShieldHealthRepairText`))
  ;[1 1 1] OverlapChecker
  (`Timeline|CheckForOverlapsTimeline`
    (:`Update`
      (`|ExecutionSequence`
        (:`then_0`
          (if (`PrimitiveComponent.IsOverlappingActor` (`self.GeneratorColliderPlayer`) (`self.XC4VCharacter`))
            (set `self.isPlayerShielded?` true)
            (else
              (set `self.isPlayerShielded?` false))))
        (:`then_1`
          (if (`PrimitiveComponent.IsOverlappingActor` (`self.AddinBallCollider`) (`self.XC4VCharacter`))
            (if (`/Game/XC4VCharacter/XC4VCharacter.isDrilling?` (`self.XC4VCharacter`))
              (set `self.isPlayerAdding?` true)
              (else
                (set `self.isPlayerAdding?` false)))))
        (:`then_2`
          (if (`PrimitiveComponent.IsOverlappingActor` (`self.AddinBallColliderInstruct`) (`self.XC4VCharacter`))
            (`SceneComponent.SetHiddenInGame` _shieldhealthrepairtext false false)
            (`SceneComponent.K2_SetWorldRotation` (`self.ShieldHealthRepairText`) (`KismetMathLibrary.FindLookAtRotation` (`SceneComponent.K2_GetComponentLocation` (`self.ShieldHealthRepairText`)) (`SceneComponent.K2_GetComponentLocation` (`/Game/AdvancedLocomotionV3/Blueprints/ALS_BaseCharacter.FP_Camera` (`self.XC4VCharacter`)))) false false)
            (else
              (`SceneComponent.SetHiddenInGame` _shieldhealthrepairtext true false))))
        (:`then_3`
          (if (`PrimitiveComponent.IsOverlappingActor` (`self.GeneratorColliderEnemies`) null)
            (if (`/Game/XC4VCharacter/XC4VCharacter.isWavesStarted?` (`self.XC4VCharacter`))
              (set `self.isEnemyOverlapping?` true)
              (else
                (set `self.isEnemyOverlapping?` false)))))))))

(event `self.GeneratorColliderEnemies.OnComponentBeginOverlap`
  (params (OverlappedComponent :type "PrimitiveComponent Object Reference") (OtherActor :type "Actor Object Reference") (OtherComp :type "PrimitiveComponent Object Reference") (OtherBodyIndex :type Integer) (bFromSweep :type Boolean) (SweepResult :type "HitResult Structure (by ref)"))
  ;[1 1 1] Enemy Checker
  (cast `/Game/Blueprints/Enemy/BP_EnemySilo` OtherActor)
  (set `self.isEnemyOverlapping?` true))

(event `self.GeneratorColliderEnemies.OnComponentEndOverlap`
  (params (OverlappedComponent :type "PrimitiveComponent Object Reference") (OtherActor :type "Actor Object Reference") (OtherComp :type "PrimitiveComponent Object Reference") (OtherBodyIndex :type Integer))
  ;[1 1 1] Enemy Checker
  (cast `/Game/Blueprints/Enemy/BP_EnemySilo` OtherActor)
  (set `self.isEnemyOverlapping?` false))

(event `StatusChecking`
  ;[1 1 1] ShieldHealthManagement
  (`Timeline|StatusCheckingTimeline`
    (:`Update`
      (`|ExecutionSequence`
        (:`then_0`
          (if (`self.isPlayerAdding?`)
            (`self.AddHealth` 5.0)))
        (:`then_1`
          (if (`self.isEnemyOverlapping?`)
            (`self.SubtractHealth` (`KismetMathLibrary.RandomFloatInRange` 0.1 0.35))))
        (:`then_2`
          (if (<= (`self.ShieldHealth`) 0.0)
            (`GameplayStatics.SpawnSound2D` "/Game/Audio/AC/ShieldShuttingDown_Cue.ShieldShuttingDown_Cue" 1.0 1.0 0.0 null :!label _label)
            (`SceneComponent.SetHiddenInGame` (`self.GeneratedShield`) true false)
            (`SceneComponent.SetHiddenInGame` (`self.GeneratedShieldGlass`) true false)))))))

(event `AddHealth`
  (params (ShieldHealthAmntAdjust :type "Float (double-precision)"))
  ;[1 1 1] ShieldHealthManagement
  (set `self.ShieldHealthAddAdjust` ShieldHealthAmntAdjust)
  (if (<= (+ (`self.ShieldHealth`) (`self.ShieldHealthAddAdjust`)) 1000.0)
    (set `self.ShieldHealth` (+ (`self.ShieldHealth`) (`self.ShieldHealthAddAdjust`)))
    (else
      (set `self.ShieldHealth` 1000.0))))

(event `SubtractHealth`
  (params (ShieldHealthSubtractAdjust :type "Float (double-precision)"))
  ;[1 1 1] ShieldHealthManagement
  (set `self.ShieldHealthSubtractAdjust` ShieldHealthSubtractAdjust)
  (if (>= (- (`self.ShieldHealth`) (`self.ShieldHealthSubtractAdjust`)) 0.0)
    (set `self.ShieldHealth` (- (`self.ShieldHealth`) (`self.ShieldHealthSubtractAdjust`)))))

(event `self.GeneratorCollider.OnComponentBeginOverlap`
  (params (OverlappedComponent :type "PrimitiveComponent Object Reference") (OtherActor :type "Actor Object Reference") (OtherComp :type "PrimitiveComponent Object Reference") (OtherBodyIndex :type Integer) (bFromSweep :type Boolean) (SweepResult :type "HitResult Structure (by ref)"))
  ;[1 1 1] ShieldHealthManagement
  (cast `/Game/XC4VCharacter/XC4VCharacter` OtherActor)
  (goto _label))

(event `RotateTexttoPlayer`
  ;[1 1 1] Health Display
  (`Timeline|RotateTexttoPlayerTimeline`
    (:`Update`
      (`SceneComponent.K2_SetWorldRotation` (`self.ShieldHealthText`) (`KismetMathLibrary.FindLookAtRotation` (`SceneComponent.K2_GetComponentLocation` (`self.ShieldHealthText`)) (`SceneComponent.K2_GetComponentLocation` (`/Game/AdvancedLocomotionV3/Blueprints/ALS_BaseCharacter.FP_Camera` (`self.XC4VCharacter`)))) false false))))

(event `SetText`
  ;[1 1 1] Health Display
  (`Timeline|SetTextTimeline`
    (:`Update`
      (`TextRenderComponent.K2_SetText` (`self.ShieldHealthText`) (`KismetTextLibrary.Conv_StringToText` (`KismetStringLibrary.Concat_StrStr` "Shield Health: " (`KismetStringLibrary.Conv_IntToString` (`KismetMathLibrary.FTrunc` (`self.ShieldHealth`))) "/1000"))))))

(event `WaveWarning`
  (bind (_glassred_r _glassred_g _glassred_b) (break `LinearColor` (`self.GlassRed`)))
  (bind (_glassblue_r _glassblue_g _glassblue_b) (break `LinearColor` (`self.GlassBlue`)))
  ;[1 1 1] WaveWarning
  (`Timeline|WaveWarningTimeline`
    (:`Update`
      (if (`/Game/XC4VCharacter/XC4VCharacter.isWavesStarted?` (`self.XC4VCharacter`))
        (bind (_direction _glasswarningtimelinecurve) (`Timeline|GlassWarningTimeline`)
          (:`Update`
            (`|ExecutionSequence`
              (:`then_0`
                (bind (_returnvalue_x _returnvalue_y _returnvalue_z) (`KismetMathLibrary.BreakVector` (`KismetMathLibrary.VLerp` (`KismetMathLibrary.MakeVector` _glassred_r _glassred_g _glassred_b) (`KismetMathLibrary.MakeVector` _glassblue_r _glassblue_g _glassblue_b) _glasswarningtimelinecurve)))
                (`MaterialInstanceDynamic.SetVectorParameterValue` (`self.ShieldGlassDynMaterial`) "ColorGlass" (make `LinearColor` _returnvalue_x _returnvalue_y _returnvalue_z 1.0))))))
        (else
          (`MaterialInstanceDynamic.SetVectorParameterValue` (`self.ShieldGlassDynMaterial`) "ColorGlass" (`self.GlassBlue`)))))))

(fn `UserConstructionScript`)