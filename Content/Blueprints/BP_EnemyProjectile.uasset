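; Enemy projectile that drains metal from the player on hit and leaves an impact actor behind.
; The Hit event subtracts MetalPickupAmnt from an XC4VCharacter's MetalAmount, spawns BP_EnemyProjectileImpact with that amount, then destroys itself.
; Other hits spawn the same impact at the hit location without draining metal, except hits on BP_EnemyTurret, which are ignored.
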(event `self.ReceiveHit`
  (params (MyComp :type "PrimitiveComponent Object Reference") (Other :type "Actor Object Reference") (OtherComp :type "PrimitiveComponent Object Reference") (bSelfMoved :type Boolean) (HitLocation :type "Vector Structure") (HitNormal :type "Vector Structure") (NormalImpulse :type "Vector Structure") (Hit :type "HitResult Structure (by ref)"))
  ;[1 1 1] OnCollide
  (bind _asxc4vcharacter (cast `/Game/XC4VCharacter/XC4VCharacter` Other)
    (:`then`
      ;[1 1 1] if Player
      (`|ExecutionSequence`
        (:`then_0`
          (set `/Game/XC4VCharacter/XC4VCharacter.MetalAmount` (- (`/Game/XC4VCharacter/XC4VCharacter.MetalAmount` _asxc4vcharacter) (`self.MetalPickupAmnt`)) _asxc4vcharacter))
        (:`then_1`
          (bind _returnvalue (`|SpawnActorFromClass` "/Game/Blueprints/BP_EnemyProjectileImpact.BP_EnemyProjectileImpact_C" (`KismetMathLibrary.MakeTransform` (0.0 0.0 0.0)) "Undefined" "OverrideRootScale" null null))
          (bind _output_get (set `self.SlugImpactPoint` _returnvalue))
          (`/Game/Blueprints/BP_EnemyProjectileImpact.ChangeAmount` _output_get (`self.MetalPickupAmnt`)))
        (:`then_3`
          (`self.K2_DestroyActor`))))
    (:`CastFailed`
      (cast `/Game/Blueprints/BP_EnemyTurret` Other
        (:`CastFailed`
          ;[1 1 1] if Not Player
          (`|ExecutionSequence`
            (:`then_1`
              (bind _returnvalue_2 (`|SpawnActorFromClass` "/Game/Blueprints/BP_EnemyProjectileImpact.BP_EnemyProjectileImpact_C" (`KismetMathLibrary.MakeTransform` HitLocation) "Undefined" "OverrideRootScale" null null))
              (bind _output_get_2 (set `self.SlugImpactPoint` _returnvalue_2))
              (`/Game/Blueprints/BP_EnemyProjectileImpact.ChangeAmount` _output_get_2 (`self.MetalPickupAmnt`)))
            (:`then_3`
              (`self.K2_DestroyActor`))))))))

(fn `UserConstructionScript`)