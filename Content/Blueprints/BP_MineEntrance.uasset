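; Mine entrance actor that serves as the level's win trigger, unlocked once the player character's IsGameWin flag is set.
; It caches the player on BeginPlay and reacts when an XC4VCharacter overlaps it, showing a locked-entrance HUD message if the game is not yet won.
; Otherwise, a one-time sequence plays death and explosion effects, hides the player and gear, disables input, then shows the win screen after a delay.
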(event `self.ReceiveBeginPlay`
  ;[1 1 1] Save Player
  (bind _asxc4vcharacter (cast `/Game/XC4VCharacter/XC4VCharacter` (`GameplayStatics.GetPlayerCharacter` 0)))
  (set `self.XC4VCharacter` _asxc4vcharacter))

(event `self.ReceiveActorBeginOverlap`
  (params (OtherActor :type "Actor Object Reference"))
  ;[1 1 1] Check for Player Overlap
  (cast `/Game/XC4VCharacter/XC4VCharacter` OtherActor)
  ;[1 1 1] Check if Won
  (if (`/Game/XC4VCharacter/XC4VCharacter.isGameWin?` (`self.XC4VCharacter`))
    ;[1 1 1] Win
    (`/Engine/EditorBlueprintResources/StandardMacros.DoOnce` false
      (:`Completed`
        (`GameplayStatics.SpawnSound2D` "/Game/Audio/DeathSound_Cue.DeathSound_Cue" 1.0 1.0 0.0 null)
        (`GameplayStatics.SpawnSound2D` "/Game/StarterContent/Audio/Explosion_Cue.Explosion_Cue" 0.8 1.0 0.0 null)
        (`AddComponent|NODE_AddParticleSystemComponent-0` :`RelativeTransform` (`SceneComponent.K2_GetComponentToWorld` (`Character.Mesh` (`self.XC4VCharacter`))))
        (`SceneComponent.SetVisibility` (`Character.Mesh` (`self.XC4VCharacter`)) false false)
        (`SceneComponent.SetVisibility` (`/Game/XC4VCharacter/XC4VCharacter.BP_XC4VBackpack` (`self.XC4VCharacter`)) false false)
        (`SceneComponent.SetVisibility` (`/Game/XC4VCharacter/XC4VCharacter.BP_XC4VCannon` (`self.XC4VCharacter`)) false false)
        (`SceneComponent.SetVisibility` (`/Game/XC4VCharacter/XC4VCharacter.BP_XC4VDrill` (`self.XC4VCharacter`)) false false)
        (`self.DisableInput` (`self.XC4VCharacter`) (`GameplayStatics.GetPlayerController` 0))
        (`KismetSystemLibrary.Delay` 2.5)
        ;;[1 1 1] Spawn Win Screen
        (bind _returnvalue (`|CreateWidget` "/Game/Widgets/WinScreen.WinScreen_C"))
        (`UserWidget.AddToViewport` _returnvalue 0)))
    (else
      ;[1 1 1] Go Win Scrub
      (`/Game/Widgets/W_Info.DebugMessage` (`/Game/XC4VCharacter/XC4VCharacter.HUDInfo` (`self.XC4VCharacter`)) "Mine Entrance Locked. Defeat the Enemies to enter!" (struct :`G` 1.0 :`B` 0.018721 :`A` 1.0)))))

(fn `UserConstructionScript`)