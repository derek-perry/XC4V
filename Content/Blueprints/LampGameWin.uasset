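; LampGameWin is a lamp Blueprint whose spotlight shows whether the game has been won.
; On BeginPlay it caches the player's XC4VCharacter, applies the default light color and starts a win check.
; The check uses a timeline's update as a polling loop, setting the light green while the character's IsGameWin flag is true and to the default color otherwise.
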(event `self.ReceiveBeginPlay`
  ;[1 1 1] SavePlayer
  (bind _asxc4vcharacter (cast `/Game/XC4VCharacter/XC4VCharacter` (`GameplayStatics.GetPlayerCharacter` 0)))
  (set `self.XC4VCharacter` _asxc4vcharacter)
  ;[1 1 1] SetDefaultLightColor
  (`LightComponent.SetLightColor` (`self.SpotLight`) (`self.DefaultLightColor`) true)
  ;[1 1 1] Init Win Checker
  (`self.CheckforWin`))

(event `CheckforWin`
  ;[1 1 1] Win Checker
  (`Timeline|CheckForWinTimeline`
    (:`Update`
      (if (`/Game/XC4VCharacter/XC4VCharacter.isGameWin?` (`self.XC4VCharacter`))
        ;[1 1 1] SetGREENLightColor
        (`LightComponent.SetLightColor` (`self.SpotLight`) (`self.GreenLightColor`) true)
        (else
          ;[1 1 1] SetDefaultLightColor
          (`LightComponent.SetLightColor` (`self.SpotLight`) (`self.DefaultLightColor`) true))))))

(fn `UserConstructionScript`)