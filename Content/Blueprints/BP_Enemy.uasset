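; Enemy actor that chases the player while the character's IsEnemying flag is set.
; Tick polls that flag; outer and inner sphere begin-overlaps set awareness and too-close flags, driving yaw tracking and swept forward steps.
; A hit while CanBeHit is true spawns an explosion, then resets the enemy to its starting transform after a short delay.
; The freeze logic that sets CanBeHit is unconnected and never runs.
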(event `self.ReceiveTick`
  (params (DeltaSeconds :type "Float (single-precision)"))
  (bind _returnvalue (`GameplayStatics.GetPlayerCharacter` 0))
  (bind _defaultsceneroot (`self.DefaultSceneRoot`))
  (bind (_returnvalue_roll _returnvalue_pitch) (`KismetMathLibrary.BreakRotator` (`SceneComponent.K2_GetComponentRotation` _defaultsceneroot)))
  (bind (_returnvalue_roll_2 _returnvalue_pitch_2 _returnvalue_yaw) (`KismetMathLibrary.BreakRotator` (`KismetMathLibrary.FindLookAtRotation` (`self.K2_GetActorLocation`) (`self.K2_GetActorLocation` _returnvalue))))
  ;[1 1 1] Everytick
  (`|ExecutionSequence`
    (:`then_1`
      ;[1 1 1] Activaly Move enemy towards player if player is in range
      ;;[1 1 1] IsWithinEnemyArea
      (if (`self.CanEnemy?`)
        ;;[1 1 1] Set Meshes Material to Active
        (`PrimitiveComponent.SetMaterial` (`self.SM_MatPreviewMesh_02`) 0 "/Game/Materials/M_MaterialSphere_Red.M_MaterialSphere_Red")
        ;;[1 1 1] Check if Player is within Enemy See Range
        (if (`self.OverlappingChar?`)
          (`|ExecutionSequence`
            (:`then_0`
              ;;[1 1 1] If Player is Too Close, Don't Move
              ;;;[1 1 1] Check if Player is Too Close
              (if (`self.TooClose?`)
                (goto _label :!via `Close`)
                (else
                  (`|ExecutionSequence`
                    (:`then_0`
                      (goto _label :!via `Open`))
                    (:`then_1`
                      (`/Engine/EditorBlueprintResources/StandardMacros.Gate` true :!label _label
                        (:`Exit`
                          ;[1 1 1] Set Location towards Player
                          (`SceneComponent.K2_SetWorldLocation` _defaultsceneroot (+ (`SceneComponent.K2_GetComponentLocation` _defaultsceneroot) (* (`SceneComponent.GetForwardVector` _defaultsceneroot) 2.0)) true false))))))))
            (:`then_1`
              ;[1 1 1] Set Rotation toward Player
              (cast `/Game/Character/XC4VCharacter` _returnvalue)
              (`SceneComponent.K2_SetWorldRotation` _defaultsceneroot (`KismetMathLibrary.MakeRotator` _returnvalue_roll _returnvalue_pitch _returnvalue_yaw) false false))))))
    (:`then_2`
      ;[1 1 1] Check if Character is in an Enemy Area
      (bind _asxc4vcharacter (cast `/Game/Character/XC4VCharacter` (`GameplayStatics.GetPlayerCharacter` 0)))
      (set `self.CanEnemy?` (`/Game/Character/XC4VCharacter.isEnemying` _asxc4vcharacter)))))

(event `self.ReceiveBeginPlay`
  ;[1 1 1] BeginPlay
  ;[1 1 1] Save Enemy's Inital Pos
  (set `self.InitialEnemyMeshTransform` (`SceneComponent.K2_GetComponentToWorld` (`self.DefaultSceneRoot`))))

(event `ResetEnemyPos`
  ;[1 1 1] Reset enemy pos to initial pos
  (`SceneComponent.K2_SetWorldTransform` (`self.DefaultSceneRoot`) (`self.InitialEnemyMeshTransform`) false true)
  (`PrimitiveComponent.SetMaterial` (`self.SM_MatPreviewMesh_02`) 0 "/Game/Materials/M_MaterialSphere_Red.M_MaterialSphere_Red")
  (`self.K2_DestroyActor` (`self.SpawnedExplosion`)))

(event `self.SM_MatPreviewMesh_02.OnComponentHit`
  (params (HitComponent :type "PrimitiveComponent Object Reference") (OtherActor :type "Actor Object Reference") (OtherComp :type "PrimitiveComponent Object Reference") (NormalImpulse :type "Vector Structure") (Hit :type "HitResult Structure (by ref)"))
  ;[1 1 1] Did The Character Collide?
  (`|ExecutionSequence`
    (:`then_1`
      (if (`self.CanEnemy?`)
        ;;[1 1 1] If Enemy CanBeHit, FatalBlow!
        (if (`self.CanBeHit?`)
          (`self.FatalBlow`))))))

(event `self.SphereInner.OnComponentBeginOverlap`
  (params (OverlappedComponent :type "PrimitiveComponent Object Reference") (OtherActor :type "Actor Object Reference") (OtherComp :type "PrimitiveComponent Object Reference") (OtherBodyIndex :type Integer) (bFromSweep :type Boolean) (SweepResult :type "HitResult Structure (by ref)"))
  ;[1 1 1] Check if too close
  (`|ExecutionSequence`
    (:`then_0`
      (cast `/Game/Character/XC4VCharacter` OtherActor
        (:`then`
          (set `self.TooClose?` true))
        (:`CastFailed`
          (set `self.TooClose?` false))))))

(event `self.SphereOuter.OnComponentBeginOverlap`
  (params (OverlappedComponent :type "PrimitiveComponent Object Reference") (OtherActor :type "Actor Object Reference") (OtherComp :type "PrimitiveComponent Object Reference") (OtherBodyIndex :type Integer) (bFromSweep :type Boolean) (SweepResult :type "HitResult Structure (by ref)"))
  ;[1 1 1] Check if within "sphere of awareness"
  (`|ExecutionSequence`
    (:`then_0`
      (cast `/Game/Character/XC4VCharacter` OtherActor
        (:`then`
          (set `self.OverlappingChar?` true))
        (:`CastFailed`
          (set `self.OverlappingChar?` false))))))

(event `FatalBlow`
  ;[1 1 1] OnEnemyHit During CanBeHit (FatalBlow)
  (`PrimitiveComponent.SetMaterial` (`self.SM_MatPreviewMesh_02`) 0 "/Game/Materials/M_MaterialSphere_Explodey.M_MaterialSphere_Explodey")
  (bind _returnvalue (`|SpawnActorFromClass` "/Game/StarterContent/Blueprints/Blueprint_Effect_Explosion.Blueprint_Effect_Explosion_C" (`SceneComponent.K2_GetComponentToWorld` (`self.SM_MatPreviewMesh_02`)) "Undefined" "OverrideRootScale" null null))
  (set `self.SpawnedExplosion` _returnvalue)
  (`KismetSystemLibrary.RetriggerableDelay` 0.3)
  (`self.ResetEnemyPos`))

(fn `UserConstructionScript`)