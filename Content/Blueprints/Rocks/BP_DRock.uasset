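; BP_DRock is a destructible rock that acts as short-lived debris, apparently left after the player drills a rock.
; On BeginPlay it caches the player's XC4VCharacter, adds an audio component, clears the character's drilling flags and destroys itself after a brief delay.
; When its destructible component is hit, it applies a small radial impulse at the impact point to that component and the hit component.
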(event `self.ReceiveBeginPlay`
  (bind _xc4vcharacter (`self.XC4VCharacter`))
  ;[1 1 1] BeginPlay
  (`|ExecutionSequence`
    (:`then_0`
      ;[1 1 1] GetPlayerChar
      (bind _asxc4vcharacter (cast `/Game/XC4VCharacter/XC4VCharacter` (`GameplayStatics.GetPlayerCharacter` 0)))
      (set `self.XC4VCharacter` _asxc4vcharacter))
    (:`then_1`
      (`AddComponent|NODE_AddAudioComponent-0`))
    (:`then_2`
      (set `/Game/XC4VCharacter/XC4VCharacter.isDrillingRock?` false _xc4vcharacter)
      (set `/Game/XC4VCharacter/XC4VCharacter.isDrilling?` false _xc4vcharacter))
    (:`then_3`
      (`KismetSystemLibrary.RetriggerableDelay` 5.0)
      (`self.K2_DestroyActor`))))

(event `self.DestructibleComponent.OnComponentHit`
  (params (HitComponent :type "PrimitiveComponent Object Reference") (OtherActor :type "Actor Object Reference") (OtherComp :type "PrimitiveComponent Object Reference") (NormalImpulse :type "Vector Structure") (Hit :type "HitResult Structure (by ref)"))
  ;[1 1 1] Do Some Impulsing
  (`PrimitiveComponent.AddRadialImpulse` (`self.DestructibleComponent`) Hit_ImpactPoint 25.0 125.0 "RIF_Constant" false)
  (`PrimitiveComponent.AddRadialImpulse` HitComponent Hit_ImpactPoint 25.0 125.0 "RIF_Constant" false))

(fn `UserConstructionScript`)