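; Minable rock that the XC4V player character drills to collect metal.
; Tick checks player overlap and drilling state, flags the character as drilling rock, then waits the character's drill time before passing a Gate.
; On completion it spawns BP_DRock, awards metal, and hides itself without collision.
; After a fixed delay it spawns a fresh copy at the saved transform and destroys itself.
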(event `self.ReceiveBeginPlay`
  ;[1 1 1] BeginPlay
  (`|ExecutionSequence`
    (:`then_1`
      ;[1 1 1] Get/Set XC4V PlayerCharacter
      (bind _asxc4vcharacter (cast `/Game/XC4VCharacter/XC4VCharacter` (`GameplayStatics.GetPlayerCharacter` 0)))
      (set `self.XC4VCharacter` _asxc4vcharacter))
    (:`then_2`
      ;[1 1 1] Save Rock Location
      (set `self.RockLocation` (`SceneComponent.K2_GetComponentToWorld` (`self.SM_Rock`))))))

(event `self.ReceiveTick`
  (params (DeltaSeconds :type "Float (single-precision)"))
  (bind _xc4vcharacter (`self.XC4VCharacter`))
  ;[1 1 1] EveryTick
  (`|ExecutionSequence`
    (:`then_0`
      ;[1 1 1] Check Player overlap while drilling for true replace
      (if (`PrimitiveComponent.IsOverlappingActor` (`self.RockCollider`) (`self.XC4VCharacter`))
        (if (`/Game/XC4VCharacter/XC4VCharacter.isDrilling?` (`self.XC4VCharacter`))
          (`|ExecutionSequence`
            (:`then_0`
              (goto _label :!via `Open`))
            (:`then_1`
              (set `/Game/XC4VCharacter/XC4VCharacter.isDrillingRock?` true (`self.XC4VCharacter`)))
            (:`then_2`
              (`KismetSystemLibrary.Delay` (`self.DrillTime`))
              (if (`self.IsOverlapping`)
                (`/Engine/EditorBlueprintResources/StandardMacros.Gate` true :!label _label
                  (:`Exit`
                    (`|SpawnActorFromClass` "/Game/Blueprints/Rocks/BP_DRock.BP_DRock_C" (`SceneComponent.K2_GetComponentToWorld` (`self.SM_Rock`)) "AlwaysSpawn" "OverrideRootScale" null null)
                    (`/Game/XC4VCharacter/XC4VCharacter.MetalPickup` _xc4vcharacter (`/Game/XC4VCharacter/XC4VCharacter.MetalPickupAmount` _xc4vcharacter))
                    (`SceneComponent.SetVisibility` (`self.SM_Rock`) false true)
                    (`self.SetActorEnableCollision` false)
                    (`KismetSystemLibrary.RetriggerableDelay` 10.0)
                    (`|SpawnActorFromClass` "BP_RockStandar_C" (`self.RockLocation`) "AlwaysSpawn" "OverrideRootScale" null null)
                    (set `/Game/XC4VCharacter/XC4VCharacter.isDrillingRock?` false (`self.XC4VCharacter`))
                    (`self.K2_DestroyActor`)))
                (else
                  (set `/Game/XC4VCharacter/XC4VCharacter.isDrillingRock?` false (`self.XC4VCharacter`))))))
          (else
            (`|ExecutionSequence`
              (:`then_0`
                (goto _label :!via `Close`))
              (:`then_1`
                (set `/Game/XC4VCharacter/XC4VCharacter.isDrillingRock?` false (`self.XC4VCharacter`))))))))
    (:`then_1`
      ;[1 1 1] Get/Set DrillTime
      (set `self.DrillTime` (`/Game/XC4VCharacter/XC4VCharacter.DrillingTime` (`self.XC4VCharacter`))))))

(event `self.RockCollider.OnComponentBeginOverlap`
  (params (OverlappedComponent :type "PrimitiveComponent Object Reference") (OtherActor :type "Actor Object Reference") (OtherComp :type "PrimitiveComponent Object Reference") (OtherBodyIndex :type Integer) (bFromSweep :type Boolean) (SweepResult :type "HitResult Structure (by ref)"))
  ;[1 1 1] Begin/End Overlap States
  (set `self.IsOverlapping` true))

(event `self.RockCollider.OnComponentEndOverlap`
  (params (OverlappedComponent :type "PrimitiveComponent Object Reference") (OtherActor :type "Actor Object Reference") (OtherComp :type "PrimitiveComponent Object Reference") (OtherBodyIndex :type Integer))
  ;[1 1 1] Begin/End Overlap States
  (set `self.IsOverlapping` false))

(fn `UserConstructionScript`)