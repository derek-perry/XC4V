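; BP_XC4VDrill is the player's drill, whose material displays how frozen it is based on the character's temperature.
; On BeginPlay it caches the XC4V player character, creates a dynamic instance of the drill mesh's material and starts SetMaterialDisplay.
; That event plays a timeline used as an update ticker, writing the inverted, offset TemperatureAmnt to the material's FrozenAmnt parameter on each update.
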(event `self.ReceiveBeginPlay`
  (bind _drillmat (`self.DrillMat`))
  ;[1 1 1] BeginPlay
  (`|ExecutionSequence`
    (:`then_0`
      ;[1 1 1] SavePlayer
      (bind _asxc4vcharacter (cast `/Game/XC4VCharacter/XC4VCharacter` (`GameplayStatics.GetPlayerCharacter` 0)))
      (set `self.XC4VCharacter` _asxc4vcharacter))
    (:`then_2`
      ;[1 1 1] Create Dynamic Backpack Material
      (set `self.DrillMat` (`PrimitiveComponent.GetMaterial` (`self.xc4vdrill`) 0))
      (bind _returnvalue (`KismetMaterialLibrary.CreateDynamicMaterialInstance` _drillmat _drillmat "DynDrillMat"))
      (set `self.DynDrillMat` _returnvalue)
      (`PrimitiveComponent.SetMaterial` (`self.xc4vdrill`) 0 (`self.DynDrillMat`)))
    (:`then_3`
      ;[1 1 1] StartingSettingMaterialDisplay
      (`self.SetMaterialDisplay`))))

(event `SetMaterialDisplay`
  ;[1 1 1] Set Material Display
  (`Timeline|Timeline_0`
    (:`Update`
      ;;[1 1 1] Temp
      (bind _output_get (set `self.TempLevelAmount` (`/Game/XC4VCharacter/XC4VCharacter.TemperatureAmnt` (`self.XC4VCharacter`))))
      (`MaterialInstanceDynamic.SetScalarParameterValue` (`self.DynDrillMat`) "FrozenAmnt" (+ (- 1.0 _output_get) 0.333333)))))

(fn `UserConstructionScript`)