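; BP_StandardRock is a rock actor that gives way when the player character drills into it.
; Each tick it checks whether player 0's XC4VCharacter overlaps the RockCollider while IsDrilling is set.
; When both hold, it spawns a BP_DRock at the SMRock mesh's world transform and destroys itself, a simple swap that polls rather than using overlap events.
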(event `self.ReceiveTick`
  (params (DeltaSeconds :type "Float (single-precision)"))
  (bind _asxc4vcharacter (cast `/Game/XC4VCharacter/XC4VCharacter` (`GameplayStatics.GetPlayerCharacter` 0)))
  (if (`PrimitiveComponent.IsOverlappingActor` (`self.RockCollider`) _asxc4vcharacter)
    (if (`/Game/XC4VCharacter/XC4VCharacter.isDrilling?` _asxc4vcharacter)
      (`|ExecutionSequence`
        (:`then_0`
          (`|SpawnActorFromClass` "/Game/Blueprints/BP_DRock.BP_DRock_C" (`SceneComponent.K2_GetComponentToWorld` (`self.SM_Rock`)) "AlwaysSpawn" "OverrideRootScale" null null))
        (:`then_1`
          (`self.K2_DestroyActor`))))))

(fn `UserConstructionScript`)