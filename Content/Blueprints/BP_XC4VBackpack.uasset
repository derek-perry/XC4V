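; BP_XC4VBackpack is the player's backpack, which visually displays the XC4V character's metal and temperature levels.
; BeginPlay caches the player character and creates dynamic material instances for the backpack and both meters.
; A timeline's Update reads MetalAmount and TemperatureAmnt from the character and writes inverted values to the meter materials.
; Temperature also drives an offset FrozenAmnt parameter on the backpack material.
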(event `self.ReceiveBeginPlay`
  (bind _backpacklavamaterial (`self.BackpackLavaMaterial`))
  (bind _backpackmat (`self.BackpackMat`))
  (bind _backpacktempmaterial (`self.BackpackTempMaterial`))
  ;[1 1 1] BeginPlay
  (`|ExecutionSequence`
    (:`then_0`
      ;[1 1 1] SavePlayer
      (bind _asxc4vcharacter (cast `/Game/XC4VCharacter/XC4VCharacter` (`GameplayStatics.GetPlayerCharacter` 0)))
      (set `self.XC4VCharacter` _asxc4vcharacter))
    (:`then_1`
      ;[1 1 1] SetMaterial
      (set `self.BackpackLavaMaterial` (`PrimitiveComponent.GetMaterial` (`self.MetalMeter`) 0))
      (bind _returnvalue (`KismetMaterialLibrary.CreateDynamicMaterialInstance` _backpacklavamaterial _backpacklavamaterial "DynBackPackLavaMat"))
      (set `self.DynamicBackpackLavaMat` _returnvalue)
      (set `self.BackpackTempMaterial` (`PrimitiveComponent.GetMaterial` (`self.TemperatureMeter`) 0))
      (bind _returnvalue_2 (`KismetMaterialLibrary.CreateDynamicMaterialInstance` _backpacktempmaterial _backpacktempmaterial "DynBackPackTempMat"))
      (set `self.DynamicBackpackTempMat` _returnvalue_2)
      (`PrimitiveComponent.SetMaterial` (`self.MetalMeter`) 0 (`self.DynamicBackpackLavaMat`))
      (`PrimitiveComponent.SetMaterial` (`self.TemperatureMeter`) 0 (`self.DynamicBackpackTempMat`)))
    (:`then_2`
      ;[1 1 1] Create Dynamic Backpack Material
      (set `self.BackpackMat` (`PrimitiveComponent.GetMaterial` (`self.Backpack`) 0))
      (bind _returnvalue_3 (`KismetMaterialLibrary.CreateDynamicMaterialInstance` _backpackmat _backpackmat "DynBackpackMat"))
      (set `self.DynBackpackMat` _returnvalue_3)
      (`PrimitiveComponent.SetMaterial` (`self.Backpack`) 0 (`self.DynBackpackMat`)))
    (:`then_3`
      ;[1 1 1] StartingSettingMaterialDisplay
      (`self.SetMaterialDisplay`))))

(event `SetMaterialDisplay`
  ;[1 1 1] Set Material Display
  (`Timeline|SetMatDisplayTimeline`
    (:`Update`
      (`|ExecutionSequence`
        (:`then_0`
          ;;[1 1 1] Lava
          (bind _output_get (set `self.LavaLevelAmount` (`/Game/XC4VCharacter/XC4VCharacter.MetalAmount` (`self.XC4VCharacter`))))
          (`MaterialInstanceDynamic.SetScalarParameterValue` (`self.DynamicBackpackLavaMat`) "LavaLevelAmnt" (- 1.0 _output_get)))
        (:`then_1`
          ;;[1 1 1] Temp
          (bind _output_get_2 (set `self.TempLevelAmount` (`/Game/XC4VCharacter/XC4VCharacter.TemperatureAmnt` (`self.XC4VCharacter`))))
          (bind _returnvalue (- 1.0 _output_get_2))
          (`MaterialInstanceDynamic.SetScalarParameterValue` (`self.DynamicBackpackTempMat`) "TempLevelAmnt" _returnvalue)
          (`MaterialInstanceDynamic.SetScalarParameterValue` (`self.DynBackpackMat`) "FrozenAmnt" (+ _returnvalue 0.333333)))))))

(fn `UserConstructionScript`)