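; BP_EnemyProjectileImpact is an enemy projectile impact effect that doubles as a metal pickup for the player.
; On BeginPlay it caches the player character, starts a timeline that polls for overlap while the player is drilling, adds particle and audio components, and destroys itself after TimeToDeath.
; A successful check triggers a one-shot timeline that lerps the MetalBall to the drill, grants the adjustable metal amount, then destroys the actor.
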(event `self.ReceiveBeginPlay`
  ;[1 1 1] Begin Play
  (`/Engine/EditorBlueprintResources/StandardMacros.DoOnce` false
    (:`Completed`
      ;[1 1 1] Save Player
      (bind _asxc4vcharacter (cast `/Game/XC4VCharacter/XC4VCharacter` (`GameplayStatics.GetPlayerCharacter` 0)))
      (set `self.XC4VCharacter` _asxc4vcharacter)
      ;[1 1 1] Begin Checking if Player Picked Up
      (`self.PickupCheckforPlayer`)
      ;[1 1 1] Otherwise spawn impact effects
      (`AddComponent|NODE_AddParticleSystemComponent-0`)
      (`AddComponent|NODE_AddAudioComponent-0`)
      ;[1 1 1] And Eventually Kill Impact and Pickup
      (`KismetSystemLibrary.RetriggerableDelay` (`self.TimeToDeath`))
      (`self.K2_DestroyActor`))))

(event `ChangeAmount`
  (params (MetalPickupAmount :type "Float (double-precision)"))
  ;[1 1 1] Adjust Metal Pickup Amount on the Fly
  (set `self.MetalPickupAmount` MetalPickupAmount))

(event `PickupCheckforPlayer`
  ;[1 1 1] If Player Overlap, do Pickup
  (`Timeline|PCheck4PlayerTimeline`
    (:`Update`
      (if (`self.IsOverlappingActor` (`self.XC4VCharacter`))
        (if (`/Game/XC4VCharacter/XC4VCharacter.isDrilling?` (`self.XC4VCharacter`))
          (`self.InitPickup`))))))

(event `InitPickup`
  ;[1 1 1] Do The Picking Up
  (`/Engine/EditorBlueprintResources/StandardMacros.DoOnce` false
    (:`Completed`
      (`|ExecutionSequence`
        (:`then_0`
          ;;[1 1 1] MetalPickup Move to Player's Drill
          (bind (_direction _metalpickuptimelinecurve) (`Timeline|MetalPickupTimeline`)
            (:`Update`
              (`SceneComponent.K2_SetWorldLocation` (`self.MetalBall`) (`KismetMathLibrary.VLerp` (`SceneComponent.K2_GetComponentLocation` (`/Game/XC4VCharacter/XC4VCharacter.BP_XC4VDrill` (`self.XC4VCharacter`))) (`SceneComponent.K2_GetComponentLocation` (`self.MetalBall`)) _metalpickuptimelinecurve) true false))
            (:`Finished`
              (`|ExecutionSequence`
                (:`then_1`
                  ;;[1 1 1] Adjust Metal Amount
                  (`/Game/XC4VCharacter/XC4VCharacter.MetalPickup` (`self.XC4VCharacter`) (`self.MetalPickupAmount`)))
                (:`then_2`
                  (`self.K2_DestroyActor`))))))))))

(fn `UserConstructionScript`)