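; Trigger actor that runs a two-wave enemy encounter, started once when the player overlaps it.
; WaveStarter uses a timeline with gate and DoN to spawn a random number of BP_EnemySiloAttacker around points A or B, tracking them in Enemies.
; A timeline-driven checker prunes invalid entries, starts the larger second wave when the first empties, then announces victory via HUD messages.
; WaveProgress polls the array but takes no action.
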(event `self.ReceiveBeginPlay`
  ;[1 1 1] BeginPlay
  (`|ExecutionSequence`
    (:`then_0`
      ;[1 1 1] SavePlayer
      (bind _asxc4vcharacter (cast `/Game/XC4VCharacter/XC4VCharacter` (`GameplayStatics.GetPlayerCharacter` 0)))
      (set `self.XC4VCharacter` _asxc4vcharacter))
    (:`then_1`
      ;[1 1 1] WaveProgression
      (`self.WaveProgress`))
    (:`then_2`
      ;[1 1 1] Init Death Checker
      (`self.EnemyDeathChecker`))))

(event `self.ReceiveActorBeginOverlap`
  (params (OtherActor :type "Actor Object Reference"))
  ;[1 1 1] On Overlap of the player
  (cast `/Game/XC4VCharacter/XC4VCharacter` OtherActor)
  ;[1 1 1] Send Message
  (`/Engine/EditorBlueprintResources/StandardMacros.DoOnce` false
    (:`Completed`
      (set `/Game/XC4VCharacter/XC4VCharacter.isWavesStarted?` true (`self.XC4VCharacter`))
      (`AddComponent|NODE_AddAudioComponent-0`)
      (`AddComponent|NODE_AddAudioComponent-1`)
      (`KismetSystemLibrary.RetriggerableDelay` 5.0)
      (`/Game/Widgets/W_Info.DebugMessage` (`/Game/XC4VCharacter/XC4VCharacter.HUDInfo` (`self.XC4VCharacter`)) "First Wave Started!" (struct :`R` 1.0 :`B` 0.018721 :`A` 1.0))
      (`KismetSystemLibrary.RetriggerableDelay` 2.0)
      ;[1 1 1] Start Wave A
      (`self.WaveStarter` 6 10)
      (set `self.WaveA` true))))

(event `WaveStarter`
  (params (Min :type Integer) (Max :type Integer))
  (bind _returnvalue (`KismetMathLibrary.RandomFloatInRange` -200.0 200.0))
  (bind (_returnvalue_x _returnvalue_y _returnvalue_z) (`KismetMathLibrary.BreakVector` (`SceneComponent.K2_GetComponentLocation` (`self.B`))))
  (bind _returnvalue_2 (- (`self.RandomEnemyCount`) 1))
  (bind (_returnvalue_x_2 _returnvalue_y_2 _returnvalue_z_2) (`KismetMathLibrary.BreakVector` (`SceneComponent.K2_GetComponentLocation` (`self.A`))))
  ;[1 1 1] Spawn Enemies
  (`|ExecutionSequence`
    (:`then_0`
      (goto _label :!via `Open`))
    (:`then_1`
      (`/Engine/EditorBlueprintResources/StandardMacros.Gate` true :!label _label
        (:`Exit`
          (`/Engine/EditorBlueprintResources/StandardMacros.DoOnce` false :!label _label_2
            (:`Completed`
              (set `self.RandomEnemyCount` (`KismetMathLibrary.RandomIntegerInRange` Min Max))
              (`Timeline|WaveSpawnerTimeline` :!label _label_3
                (:`Update`
                  (bind _counter (`/Engine/EditorBlueprintResources/StandardMacros.Do N` _returnvalue_2 :!label _label_4)
                    (:`Exit`
                      (if (>= _counter _returnvalue_2)
                        (set `self.EnemySpawnedCount` (stale _returnvalue_4))
                        ;;[1 1 1] Resetter
                        (`|ExecutionSequence`
                          (:`then_0`
                            (goto _label_3 :!via `Stop`))
                          (:`then_1`
                            (goto _label :!via `Close`))
                          (:`then_2`
                            (goto _label_4 :!via `Reset`))
                          (:`then_3`
                            (goto _label_2 :!via `Reset`)))
                        (else
                          (bind _returnvalue_3 (`|SpawnActorFromClass` "/Game/Blueprints/Enemy/BP_EnemySiloAttacker.BP_EnemySiloAttacker_C" (`KismetMathLibrary.MakeTransform` (select `int` (`KismetMathLibrary.RandomIntegerInRange` 0 1) :`0` (`KismetMathLibrary.MakeVector` (+ _returnvalue_x_2 _returnvalue) (+ _returnvalue_y_2 _returnvalue) (+ _returnvalue_z_2 _returnvalue)) :`1` (`KismetMathLibrary.MakeVector` (+ _returnvalue_x _returnvalue) (+ _returnvalue_y _returnvalue) (+ _returnvalue_z _returnvalue)))) "AlwaysSpawn" "OverrideRootScale" null null))
                          (bind _returnvalue_4 (`KismetArrayLibrary.Array_Add` (`self.Enemies`) _returnvalue_3)))))))))))))))

(event `WaveProgress`
  ;[1 1 1] Wave Progression
  (`Timeline|WaveProgressTimeline`
    (:`Update`
      (if (<= (`KismetArrayLibrary.Array_Length` (`self.Enemies`)) 0)
        _
        (elif (>= (`KismetArrayLibrary.Array_Length` (`self.Enemies`)) 1)
          _)))))

(event `EnemyDeathChecker`
  ;[1 1 1] Enemy Death Checker
  (`Timeline|EnemyDeathCheckerTimeline`
    (:`Update`
      (`|ExecutionSequence`
        (:`then_0`
          ;;[1 1 1] Cleanup Enemy Array
          (for (_array_element _array_index) (`self.Enemies`)
            (if (not (`KismetSystemLibrary.IsValid` _array_element))
              (`KismetArrayLibrary.Array_Remove` (`self.Enemies`) _array_index))))
        (:`then_1`
          ;;[1 1 1] Wave A
          (if (`self.WaveA`)
            (if (<= (`KismetArrayLibrary.Array_Length` (`self.Enemies`)) 0)
              (set `self.WaveA` false)
              (`/Game/Widgets/W_Info.DebugMessage` (`/Game/XC4VCharacter/XC4VCharacter.HUDInfo` (`self.XC4VCharacter`)) "First Wave Defeated!" (struct :`G` 1.0 :`B` 0.018721 :`A` 1.0))
              ;;[1 1 1] Wave A->B Transition
              (`KismetSystemLibrary.RetriggerableDelay` 1.69)
              (`AddComponent|NODE_AddAudioComponent-2`)
              (`KismetSystemLibrary.RetriggerableDelay` 5.0)
              (`self.WaveStarter` 10 15)
              (set `self.WaveB` true)
              (`/Game/Widgets/W_Info.DebugMessage` (`/Game/XC4VCharacter/XC4VCharacter.HUDInfo` (`self.XC4VCharacter`)) "Second Wave Started!" (struct :`R` 1.0 :`B` 0.018721 :`A` 1.0)))
            (else
              ;;[1 1 1] Wave B
              (if (`self.WaveB`)
                (if (<= (`KismetArrayLibrary.Array_Length` (`self.Enemies`)) 0)
                  (set `self.WaveB` false)
                  (`/Game/Widgets/W_Info.DebugMessage` (`/Game/XC4VCharacter/XC4VCharacter.HUDInfo` (`self.XC4VCharacter`)) "Second Wave Defeated! \nCongratulations!" (struct :`G` 1.0 :`B` 0.018721 :`A` 1.0)))))))))))

(fn `UserConstructionScript`)