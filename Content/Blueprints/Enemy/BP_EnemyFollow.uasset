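; Hovering enemy bot that chases the player within its interact radius and trades knockback on contact.
; Timelines act as update loops for proximity, attacks, hammer hits, hover, state materials and health.
; Spray and slug impacts freeze it temporarily, halting movement via a move-to-self.
; Hammer hits injure it, or kill it outright when frozen; death posts a HUD message, adds particles and audio, then destroys the actor.
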(event `self.ReceiveBeginPlay`
  ;[1 1 1] Begin Play
  (`|ExecutionSequence`
    (:`then_0`
      ;[1 1 1] SaveEnemySpawnPoint
      (set `self.EnemySpawnPoint` (`self.GetTransform`))
      ;[1 1 1] Save Player
      (bind _asxc4vcharacter (cast `/Game/XC4VCharacter/XC4VCharacter` (`GameplayStatics.GetPlayerCharacter` 0)))
      (set `self.XC4VCharacter` _asxc4vcharacter)
      ;[1 1 1] Start Checking for Player
      (`self.CheckPlayerNearEnemy`)
      ;[1 1 1] Init HammerHitChecker
      (`self.HammerHitCheck`)
      ;[1 1 1] Init EnemyCheck
      (`self.EnemyCheck`))
    (:`then_1`
      ;[1 1 1] Init Enemy Hover
      (`self.EnemyHover`))
    (:`then_2`
      ;[1 1 1] InitSensePlayer
      (`self.SensePlayer`))))

(event `self.PawnSensing.OnSeePawn`
  (params (Pawn :type "Pawn Object Reference"))
  ;[1 1 1] On Sense Player, Follow Player
  (cast `/Game/XC4VCharacter/XC4VCharacter` Pawn)
  (if (`self.isFrozen?`) :!label _label
    ;;[1 1 1] Move To Self/STOP
    (`|AIMoveTo` (`self.PawnSensing`) self (0.0 0.0 0.0) self 25.0 true :!label _label_2)
    (else
      ;;[1 1 1] Move To Character/Player
      (`|AIMoveTo` (`self.PawnSensing`) self (0.0 0.0 0.0) (`self.XC4VCharacter`) 150.0))))

(event `SensePlayer`
  ;[1 1 1] On Sense Player, Follow Player
  (`Timeline|SensePlayerTimeline`
    (:`Update`
      (if (`self.isEnemying?`)
        (if (`PrimitiveComponent.IsOverlappingActor` (`self.AttackRadius`) (`self.XC4VCharacter`))
          (`self.EnemyKnockback` 10000.0)
          (`/Game/XC4VCharacter/XC4VCharacter.PlayerKnockback` (`self.XC4VCharacter`) 15.0)
          (goto _label)
          (else
            (goto _label)))
        (else
          (goto _label_2))))))

(event `EnemyHover`
  (bind (_returnvalue_x _returnvalue_y _returnvalue_z) (`KismetMathLibrary.BreakVector` (`self.K2_GetActorLocation`)))
  ;[1 1 1] EnemyHovering
  (bind (_direction _enemyhovertimelinecurve) (`Timeline|EnemyHoverTimeline`)
    (:`Update`
      (`self.K2_SetActorLocation` (`KismetMathLibrary.MakeVector` _returnvalue_x _returnvalue_y (+ _returnvalue_z _enemyhovertimelinecurve)) true))))

(event `EnemyKnockback`
  (params (KnockBackAmnt :type "Float (double-precision)"))
  (bind _knockbackamnt (`self.KnockBackAmnt`))
  (bind (_returnvalue_x _returnvalue_y _returnvalue_z) (`KismetMathLibrary.BreakVector` (* (`SceneComponent.GetForwardVector` (`self.CapsuleComponent`)) -1.0)))
  ;[1 1 1] Knockback the Enemy
  (set `self.KnockBackAmnt` KnockBackAmnt)
  (`CharacterMovementComponent.AddImpulse` (`self.CharacterMovement`) (`KismetMathLibrary.MakeVector` (* _returnvalue_x _knockbackamnt) (* _returnvalue_y _knockbackamnt) (* _returnvalue_z _knockbackamnt)) true))

(event `self.HitImpactRadius.OnComponentBeginOverlap`
  (params (OverlappedComponent :type "PrimitiveComponent Object Reference") (OtherActor :type "Actor Object Reference") (OtherComp :type "PrimitiveComponent Object Reference") (OtherBodyIndex :type Integer) (bFromSweep :type Boolean) (SweepResult :type "HitResult Structure (by ref)"))
  ;[1 1 1] OnSprayHit
  (cast `/Game/Blueprints/BP_SprayImpact` (stale `self.SlugImpactRadius.OnComponentBeginOverlap` OtherActor) :!label _label_3
    (:`then`
      (if (not (`self.isFrozen?`))
        (`|ExecutionSequence`
          (:`then_0`
            (set `self.isFrozen?` true)
            (`PrimitiveComponent.SetMaterial` (`self.Enemy`) 0 (`self.FrozenMaterial`))
            (`self.EnemyKnockback` 5000.0))
          (:`then_1`
            (`self.EnemyKnockback` 500.0))
          (:`then_3`
            (`KismetSystemLibrary.RetriggerableDelay` (`self.FrozenTime`))
            (if (`self.isFrozen?`)
              (set `self.isFrozen?` false)
              (`|ExecutionSequence`
                (:`then_1`
                  ;[1 1 1] Check for Enemy States and update Enemy
                  ;;[1 1 1] Active/Enemying
                  (if (`self.isEnemying?`) :!label _label_4
                    ;;[1 1 1] Frozen
                    (if (`self.isFrozen?`)
                      (`PrimitiveComponent.SetMaterial` (`self.Enemy`) 0 (`self.FrozenMaterial`))
                      (else
                        ;;[1 1 1] Injury/Ouch
                        (if (`self.isOuch?`)
                          (`PrimitiveComponent.SetMaterial` (`self.Enemy`) 0 (`self.OuchMaterial`))
                          (else
                            ;;[1 1 1] Dieing
                            (if (`self.isDieing?`)
                              (`PrimitiveComponent.SetMaterial` (`self.Enemy`) 0 (`self.DieMaterial`))
                              (else
                                (`PrimitiveComponent.SetMaterial` (`self.Enemy`) 0 (`self.EnemyMaterial`))))))))
                    (else
                      ;;[1 1 1] Frozen
                      (if (`self.isFrozen?`)
                        (`PrimitiveComponent.SetMaterial` (`self.Enemy`) 0 (`self.FrozenMaterial`))
                        (else
                          ;;[1 1 1] Injury/Ouch
                          (if (`self.isOuch?`)
                            (`PrimitiveComponent.SetMaterial` (`self.Enemy`) 0 (`self.OuchMaterial`))
                            (else
                              ;;[1 1 1] Dieing
                              (if (`self.isDieing?`)
                                (`PrimitiveComponent.SetMaterial` (`self.Enemy`) 0 (`self.DieMaterial`))
                                (else
                                  ;;[1 1 1] Else Grey
                                  (`PrimitiveComponent.SetMaterial` (`self.Enemy`) 0 (`self.GreyMaterial`)))))))))))))))))
    (:`CastFailed`
      (bind _asxc4vcharacter (cast `/Game/XC4VCharacter/XC4VCharacter` OtherActor))
      (if (not (`self.isKnockingBack?`))
        (`|ExecutionSequence`
          (:`then_1`
            (`/Game/XC4VCharacter/XC4VCharacter.PlayerKnockback` _asxc4vcharacter 750.0)
            (`self.EnemyKnockback` 500.0)
            (set `self.isKnockingBack?` true))
          (:`then_2`
            (`KismetSystemLibrary.RetriggerableDelay` 0.85)
            (set `self.isKnockingBack?` false)))))))

(event `self.SlugImpactRadius.OnComponentBeginOverlap`
  (params (OverlappedComponent :type "PrimitiveComponent Object Reference") (OtherActor :type "Actor Object Reference") (OtherComp :type "PrimitiveComponent Object Reference") (OtherBodyIndex :type Integer) (bFromSweep :type Boolean) (SweepResult :type "HitResult Structure (by ref)"))
  ;[1 1 1] OnSlugHit
  (cast `/Game/Blueprints/BP_SlugImpact` OtherActor
    (:`then`
      (if (not (`self.isFrozen?`))
        (`|ExecutionSequence`
          (:`then_0`
            (set `self.isFrozen?` true)
            (`PrimitiveComponent.SetMaterial` (`self.Enemy`) 0 (`self.FrozenMaterial`))
            (`self.EnemyKnockback` 5000.0))
          (:`then_1`
            (`self.EnemyKnockback` 666.0))
          (:`then_3`
            (`KismetSystemLibrary.RetriggerableDelay` (`self.FrozenTime`))
            (if (`self.isFrozen?`)
              (set `self.isFrozen?` false)
              (`|ExecutionSequence`
                (:`then_1`
                  (goto _label_4))))))))
    (:`CastFailed`
      (goto _label_3))))

(event `HammerHitCheck`
  ;[1 1 1] Check if player is Hammerhitting
  (`Timeline|HammerHitChecker`
    (:`Update`
      (if (and (`PrimitiveComponent.IsOverlappingComponent` (`self.HitImpactRadius`) (`/Game/XC4VCharacter/XC4VCharacter.HitCollider` (`self.XC4VCharacter`))) (`/Game/XC4VCharacter/XC4VCharacter.isHammering?` (`self.XC4VCharacter`)))
        (if (`self.isFrozen?`)
          (`self.EnemyKnockback` 5000.0)
          (`self.DIEZOMBIE`)
          (else
            (`self.EnemyKnockback` 5000.0)
            (`self.OUCHZOMBIE`)))))))

(event `OUCHZOMBIE`
  ;[1 1 1] Bot Injury
  (if (not (`self.isOuch?`))
    (set `self.isOuch?` true)
    (`|ExecutionSequence`
      (:`then_0`
        (`PrimitiveComponent.SetMaterial` (`self.Enemy`) 0 (`self.OuchMaterial`)))
      (:`then_1`
        (`KismetSystemLibrary.RetriggerableDelay` 0.1)
        (`|ExecutionSequence`
          (:`then_0`
            (set `self.isOuch?` false))
          (:`then_1`
            (goto _label_4))))
      (:`then_2`
        (set `self.BotHealth` (- (`self.BotHealth`) 0.5)))
      (:`then_3`
        (`self.EnemyKnockback` 750.0)))))

(event `DIEZOMBIE`
  ;[1 1 1] Bot Death
  (if (not (`self.isDieing?`))
    (set `self.isDieing?` true)
    (`PrimitiveComponent.SetMaterial` (`self.Enemy`) 0 (`self.DieMaterial`))
    ;;[1 1 1] Send Message About An Enemy being Killed
    (bind _asxc4vcharacter (cast `/Game/XC4VCharacter/XC4VCharacter` (`GameplayStatics.GetPlayerCharacter` 0)))
    (`/Game/Widgets/W_Info.DebugMessage` (`/Game/XC4VCharacter/XC4VCharacter.HUDInfo` _asxc4vcharacter) "BOT ELIMINATED!" (struct :`R` 1.0 :`G` 0.111022 :`A` 1.0))
    (`AddComponent|NODE_AddParticleSystemComponent-2`)
    (`AddComponent|NODE_AddAudioComponent-0`)
    (`SceneComponent.SetVisibility` (`self.Mesh`) false false)
    (`SceneComponent.SetVisibility` (`self.Enemy`) false false)
    (`self.SetActorEnableCollision` false)
    (`KismetSystemLibrary.RetriggerableDelay` 1.3)
    (`self.K2_DestroyActor`)))

(event `EnemyCheck`
  ;[1 1 1] Check for Enemy States and update Enemy
  (`Timeline|EnemyCheckTimeline`
    (:`Update`
      (`|ExecutionSequence`
        (:`then_1`
          (goto _label_4))
        (:`then_2`
          ;;[1 1 1] Health Death
          (if (< (`self.BotHealth`) 0.0)
            (`self.DIEZOMBIE`)))))))

(event `CheckPlayerNearEnemy`
  ;[1 1 1] Check if Player is Near Enemy
  (`Timeline|EnemyPlayerChecker`
    (:`Update`
      (if (`PrimitiveComponent.IsOverlappingActor` (`self.EnemyInteractRadius`) (`self.XC4VCharacter`))
        (set `self.isEnemying?` true)
        (else
          (set `self.isEnemying?` false)
          (goto _label_2))))))

(fn `UserConstructionScript`)