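; Enemy projectile that drains metal from the player on hit.
; The Hit event casts the other actor to XC4VCharacter and subtracts MetalPickupAmnt from its MetalAmount, ignoring anything else.
; Logic to spawn a BP_EnemyProjectileImpact carrying that amount and destroy the projectile, including a turret exclusion check, is disconnected and never runs.
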(event `self.ReceiveHit`
  (params (MyComp :type "PrimitiveComponent Object Reference") (Other :type "Actor Object Reference") (OtherComp :type "PrimitiveComponent Object Reference") (bSelfMoved :type Boolean) (HitLocation :type "Vector Structure") (HitNormal :type "Vector Structure") (NormalImpulse :type "Vector Structure") (Hit :type "HitResult Structure (by ref)"))
  ;[1 1 1] OnCollide
  (bind _asxc4vcharacter (cast `/Game/XC4VCharacter/XC4VCharacter` Other))
  ;[1 1 1] if Player
  (set `/Game/XC4VCharacter/XC4VCharacter.MetalAmount` (- (`/Game/XC4VCharacter/XC4VCharacter.MetalAmount` _asxc4vcharacter) (`self.MetalPickupAmnt`)) _asxc4vcharacter))

(fn `UserConstructionScript`)