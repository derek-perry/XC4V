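; BP_PreD is an intact stand-in for a destructible object that is replaced by a BP_D actor when an XC4VCharacter breaks it.
; On BeginPlay it applies its configured mesh and sizes the sphere collider to twice that mesh's bounding radius.
; An overlap while drilling, or a hit while drilling or hammering, spawns BP_D at the mesh's transform, aligns its mesh and destroys this actor.
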(event `self.ReceiveBeginPlay`
  ;[1 1 1] Begin Play
  (`StaticMeshComponent.SetStaticMesh` (`self.PreDMesh`) (`self.NewPreDMesh`))
  (`SphereComponent.SetSphereRadius` (`self.PreDCollider`) (* (`.SphereRadius` (`KismetSystemLibrary.GetComponentBounds` (`self.PreDMesh`))) 2.0) true))

(event `self.ReceiveActorBeginOverlap`
  (params (OtherActor :type "Actor Object Reference"))
  (bind _returnvalue (`SceneComponent.K2_GetComponentToWorld` (`self.PreDMesh`)))
  ;[1 1 1] On Overlap
  (bind _asxc4vcharacter (cast `/Game/Character/XC4VCharacter` OtherActor))
  (if (`/Game/Character/XC4VCharacter.isDrilling` _asxc4vcharacter)
    ;[1 1 1] On Collide, Spawn Destructable Version
    (bind _returnvalue_2 (`|SpawnActorFromClass` "/Game/Blueprints/BP_D.BP_D_C" _returnvalue "AlwaysSpawn" "OverrideRootScale" null null :!label _label))
    (`SceneComponent.K2_SetWorldTransform` (`/Game/Blueprints/BP_D.DMesh` _returnvalue_2) _returnvalue false false)
    (`self.K2_DestroyActor`)))

(event `self.ReceiveHit`
  (params (MyComp :type "PrimitiveComponent Object Reference") (Other :type "Actor Object Reference") (OtherComp :type "PrimitiveComponent Object Reference") (bSelfMoved :type Boolean) (HitLocation :type "Vector Structure") (HitNormal :type "Vector Structure") (NormalImpulse :type "Vector Structure") (Hit :type "HitResult Structure (by ref)"))
  ;[1 1 1] On HIT
  (bind _asxc4vcharacter (cast `/Game/Character/XC4VCharacter` Other))
  (if (`/Game/Character/XC4VCharacter.isDrilling` _asxc4vcharacter)
    (goto _label)
    (elif (`/Game/Character/XC4VCharacter.isHammer` _asxc4vcharacter)
      (goto _label))))

(fn `UserConstructionScript`)