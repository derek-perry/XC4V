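; BP_Generator is the shield generator that the player repairs by drilling inside its collider, restoring shield health up to a cap.
; Timelines act as update loops for overlap checks, health management and world-space text that faces the player camera.
; Overlap checks set the repair flag and toggle instruction text, while health management updates the character's ShieldAmnt and respawns BP_Shield with a sound when health returns.
; BeginPlay caches the player and polls until Shield and Silo references are valid.
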(event `self.ReceiveBeginPlay`
  ;[1 0 0] BeginPlay
  (`|ExecutionSequence`
    (:`then_0`
      ;[1 1 1] SavePlayer
      (bind _asxc4vcharacter (cast `/Game/XC4VCharacter/XC4VCharacter` (`GameplayStatics.GetPlayerCharacter` 0)))
      (set `self.XC4VCharacter` _asxc4vcharacter))
    (:`then_1`
      ;[1 1 1] OverlapChecker
      (`self.CheckforOverlaps`))
    (:`then_2`
      ;[1 1 1] ShieldHealthManagement
      (`|ExecutionSequence`
        (:`then_0`
          (`self.StatusChecking`))))
    (:`then_3`
      ;[1 1 1] Health Display
      (`self.SetText`))
    (:`then_4`
      (`self.RotateTexttoPlayer`))
    (:`then_6`
      ;[1 1 1] Save Shield
      (if (`KismetSystemLibrary.IsValid` (`/Game/XC4VCharacter/XC4VCharacter.Shield` (`self.XC4VCharacter`))) :!label _label
        (set `self.Shield` (`/Game/XC4VCharacter/XC4VCharacter.Shield` (`self.XC4VCharacter`)))
        (if (`KismetSystemLibrary.IsValid` (`self.Shield`))
          (set `self.ShieldLoc` (`SceneComponent.K2_GetComponentToWorld` (`/Game/Blueprints/SiloShieldStuff/BP_Shield.DefaultSceneRoot` (`self.Shield`)))))
        (else
          (`KismetSystemLibrary.Delay` 0.42)
          (goto _label))))
    (:`then_7`
      ;[1 1 1] Save Silo
      (if (`KismetSystemLibrary.IsValid` (`/Game/XC4VCharacter/XC4VCharacter.Silo` (`self.XC4VCharacter`))) :!label _label_2
        (set `self.Silo` (`/Game/XC4VCharacter/XC4VCharacter.Silo` (`self.XC4VCharacter`)))
        (if (`KismetSystemLibrary.IsValid` (`self.Silo`))
          (set `self.SiloLoc` (`SceneComponent.K2_GetComponentToWorld` (`/Game/Blueprints/SiloShieldStuff/BP_Silo.MetalSilo` (`self.Silo`)))))
        (else
          (`KismetSystemLibrary.Delay` 0.42)
          (goto _label_2))))))

(event `CheckforOverlaps`
  (bind _shieldhealthrepairtext (`self.ShieldHealthRepairText`))
  ;[1 1 1] OverlapChecker
  (`Timeline|CheckForOverlapsTimeline`
    (:`Update`
      (`|ExecutionSequence`
        (:`then_1`
          (if (`PrimitiveComponent.IsOverlappingActor` (`self.AddinBallCollider`) (`self.XC4VCharacter`))
            (if (`/Game/XC4VCharacter/XC4VCharacter.isDrilling?` (`self.XC4VCharacter`))
              (set `self.isPlayerAdding?` true)
              (else
                (set `self.isPlayerAdding?` false :!label _label_3)))
            (else
              (goto _label_3))))
        (:`then_2`
          (if (`PrimitiveComponent.IsOverlappingActor` (`self.AddinBallColliderInstruct`) (`self.XC4VCharacter`))
            (`SceneComponent.SetHiddenInGame` _shieldhealthrepairtext false false)
            (`SceneComponent.K2_SetWorldRotation` (`self.ShieldHealthRepairText`) (`KismetMathLibrary.FindLookAtRotation` (`SceneComponent.K2_GetComponentLocation` (`self.ShieldHealthRepairText`)) (`SceneComponent.K2_GetComponentLocation` (`/Game/AdvancedLocomotionV3/Blueprints/ALS_BaseCharacter.FP_Camera` (`self.XC4VCharacter`)))) false false)
            (else
              (`SceneComponent.SetHiddenInGame` _shieldhealthrepairtext true false))))))))

(event `StatusChecking`
  ;[1 1 1] ShieldHealthManagement
  (`|SpawnActorFromClass` "/Game/Blueprints/SiloShieldStuff/BP_Shield.BP_Shield_C" (`self.ShieldLoc`) "AlwaysSpawn" "OverrideRootScale" null null)
  (`Timeline|StatusCheckingTimeline`
    (:`Update`
      (`|ExecutionSequence`
        (:`then_0`
          (if (<= (`/Game/XC4VCharacter/XC4VCharacter.ShieldAmnt` (`self.XC4VCharacter`)) 2.0)
            (set `/Game/XC4VCharacter/XC4VCharacter.ShieldAmnt` 0.0 (`self.XC4VCharacter`))))
        (:`then_1`
          (set `self.Shield` (`/Game/XC4VCharacter/XC4VCharacter.Shield` (`self.XC4VCharacter`))))
        (:`then_3`
          (if (`KismetSystemLibrary.IsValid` (`self.Shield`))
            (`|ExecutionSequence`
              (:`then_1`
                (if (`self.isPlayerAdding?`)
                  (if (<= (+ (`/Game/XC4VCharacter/XC4VCharacter.ShieldAmnt` (`self.XC4VCharacter`)) (`self.SpeedFix`)) 1000.0) :!label _label_4
                    (set `/Game/XC4VCharacter/XC4VCharacter.ShieldAmnt` (+ (`/Game/XC4VCharacter/XC4VCharacter.ShieldAmnt` (`self.XC4VCharacter`)) (`self.SpeedFix`)) (`self.XC4VCharacter`))
                    (else
                      (set `/Game/XC4VCharacter/XC4VCharacter.ShieldAmnt` 1000.0 (`self.XC4VCharacter`)))))))
            (else
              (`|ExecutionSequence`
                (:`then_0`
                  (if (`self.isPlayerAdding?`)
                    (goto _label_4)))
                (:`then_1`
                  (if (not (<= (`/Game/XC4VCharacter/XC4VCharacter.ShieldAmnt` (`self.XC4VCharacter`)) 0.0))
                    (`/Engine/EditorBlueprintResources/StandardMacros.DoOnce` false :!label _label_5
                      (:`Completed`
                        (`|SpawnActorFromClass` "/Game/Blueprints/SiloShieldStuff/BP_Shield.BP_Shield_C" (`self.ShieldLoc`) "AlwaysSpawn" "OverrideRootScale" null null)
                        (`GameplayStatics.SpawnSound2D` "/Game/Audio/AC/ShieldTurningOn_1_Cue.ShieldTurningOn_1_Cue" 3.0 1.0 0.0 null)
                        (goto _label_5 :!via `Reset`)))))))))))))

(event `RotateTexttoPlayer`
  ;[1 1 1] Health Display
  (`Timeline|RotateTexttoPlayerTimeline`
    (:`Update`
      (`SceneComponent.K2_SetWorldRotation` (`self.ShieldHealthText`) (`KismetMathLibrary.FindLookAtRotation` (`SceneComponent.K2_GetComponentLocation` (`self.ShieldHealthText`)) (`SceneComponent.K2_GetComponentLocation` (`/Game/AdvancedLocomotionV3/Blueprints/ALS_BaseCharacter.FP_Camera` (`self.XC4VCharacter`)))) false false))))

(event `SetText`
  ;[1 1 1] Health Display
  (`Timeline|SetTextTimeline`
    (:`Update`
      (if (`KismetSystemLibrary.IsValid` (`self.Shield`))
        (`TextRenderComponent.K2_SetText` (`self.ShieldHealthText`) (`KismetTextLibrary.Conv_StringToText` (`KismetStringLibrary.Concat_StrStr` "Shield Health: " (`KismetStringLibrary.Conv_IntToString` (`KismetMathLibrary.FTrunc` (`/Game/XC4VCharacter/XC4VCharacter.ShieldAmnt` (`self.XC4VCharacter`)))) "/1000")))))))

(fn `UserConstructionScript`)