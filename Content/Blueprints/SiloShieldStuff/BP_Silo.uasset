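; BP_Silo is the silo players defend: enemy contact drains its metal while shields are down, and running out ends the game.
; The metal amount lives on XC4VCharacter, where the silo registers itself.
; Timeline updates drive the camera-facing percentage text, dynamic lava material and low-metal warning, and poll all enemies for collider overlap, keeping only the last result.
; Game over explodes the silo, disables input and shows GameOverScreen after a delay.
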(event `self.ReceiveBeginPlay`
  (bind _silolavamaterial (`self.SiloLavaMaterial`))
  (`|ExecutionSequence`
    (:`then_0`
      ;[1 1 1] SavePlayer and silo
      (bind _asxc4vcharacter (cast `/Game/XC4VCharacter/XC4VCharacter` (`GameplayStatics.GetPlayerCharacter` 0)))
      (set `self.XC4VCharacter` _asxc4vcharacter))
    (:`then_1`
      ;[1 1 1] Get and Set Material for Lava amount
      (set `self.SiloLavaMaterial` (`PrimitiveComponent.GetMaterial` (`self.MetalSilo`) 0))
      (bind _returnvalue (`KismetMaterialLibrary.CreateDynamicMaterialInstance` _silolavamaterial _silolavamaterial "DynSiloLavaMat"))
      (set `self.DynamicSiloLavaMat` _returnvalue)
      (`PrimitiveComponent.SetMaterial` (`self.MetalSilo`) 0 (`self.DynamicSiloLavaMat`)))
    (:`then_2`
      ;[1 1 1] Start Setting Laval Level
      (`self.SetLavaAmnt`))
    (:`then_3`
      ;[1 1 1] Save Self as Shield
      (set `/Game/XC4VCharacter/XC4VCharacter.Silo` self (`self.XC4VCharacter`)))
    (:`then_4`
      ;[1 1 1] Init SiloMetalAdjust
      (`self.SiloMetalAdjust`))))

(event `SetLavaAmnt`
  ;[1 1 1] Set Lava Level Display
  (`Timeline|SetLavaAmntTimeline`
    (:`Update`
      (`|ExecutionSequence`
        (:`then_0`
          (`TextRenderComponent.K2_SetText` (`self.SiloHealthText`) (`KismetTextLibrary.Conv_StringToText` (`KismetStringLibrary.Concat_StrStr` (`KismetStringLibrary.Conv_IntToString` (`KismetMathLibrary.FTrunc` (* (`/Game/XC4VCharacter/XC4VCharacter.SiloMetalAmnt` (`self.XC4VCharacter`)) 100.0))) "%"))))
        (:`then_1`
          (`SceneComponent.K2_SetWorldRotation` (`self.SiloHealthText`) (`KismetMathLibrary.FindLookAtRotation` (`SceneComponent.K2_GetComponentLocation` (`self.SiloHealthText`)) (`SceneComponent.K2_GetComponentLocation` (`/Game/AdvancedLocomotionV3/Blueprints/ALS_BaseCharacter.FP_Camera` (`self.XC4VCharacter`)))) false false))
        (:`then_2`
          ;;[1 1 1] Lava amnt disaply
          (`MaterialInstanceDynamic.SetScalarParameterValue` (`self.DynamicSiloLavaMat`) "LavaLevelAmnt" (- 1.0 (`/Game/XC4VCharacter/XC4VCharacter.SiloMetalAmnt` (`self.XC4VCharacter`)))))
        (:`then_3`
          ;;[1 1 1] On Low Metal
          (if (< (`/Game/XC4VCharacter/XC4VCharacter.SiloMetalAmnt` (`self.XC4VCharacter`)) 0.3)
            (`/Engine/EditorBlueprintResources/StandardMacros.DoOnce` false :!label _label
              (:`Completed`
                (`GameplayStatics.SpawnSound2D` "/Game/Audio/AC/MetalLow_Cue.MetalLow_Cue" 8.0 1.0 0.0 null)))
            (else
              (goto _label :!via `Reset`))))
        (:`then_4`
          ;;[1 1 1] On Zero Metal
          (if (< (`/Game/XC4VCharacter/XC4VCharacter.SiloMetalAmnt` (`self.XC4VCharacter`)) 0.0)
            (`self.SiloGameOver`)))))))

(event `SiloMetalAdjust`
  ;[1 1 1] Silo Metal Level Amount Adjustments
  ;;[1 1 1] SiloMetalAdjustChecker
  (`Timeline|SiloMetalAdjustTimeline`
    (:`Update`
      (`|ExecutionSequence`
        (:`then_0`
          ;;[1 1 1] SiloLevelA,mt
          (if (> (`/Game/XC4VCharacter/XC4VCharacter.SiloMetalAmnt` (`self.XC4VCharacter`)) 0.0)
            (if true
              _)
            (elif true
              _)))
        (:`then_1`
          ;;[1 1 1] Enemyoverlap?
          (bind _outactors (`GameplayStatics.GetAllActorsOfClass` "/Game/Blueprints/Enemy/BP_EnemyMain.BP_EnemyMain_C"))
          (for _array_element _outactors
            (`/Engine/EditorBlueprintResources/StandardMacros.IsValid` _array_element
              (:`Is Valid`
                (if (`PrimitiveComponent.IsOverlappingComponent` (`Character.CapsuleComponent` _array_element) (`self.SiloCollider`))
                  (set `self.isEnemyOverlapping?` true)
                  (else
                    (set `self.isEnemyOverlapping?` false)))))))
        (:`then_3`
          ;;[1 1 1] Subtract on Enemy Overlap
          (if (`self.isEnemyOverlapping?`)
            (if (<= (`/Game/XC4VCharacter/XC4VCharacter.ShieldAmnt` (`self.XC4VCharacter`)) 0.0)
              (`self.SiloSubtracto` (`self.SiloSubtractoAmnt`)))))))))

(event `SiloSubtracto`
  (params (SiloSubtractoAmnt :type "Float (double-precision)"))
  ;[1 1 1] Silo Metal Level Amount Adjustments
  ;;[1 1 1] Subtract Silo Amnt
  (set `self.SiloSubtractoAmntSet` SiloSubtractoAmnt)
  (if (>= (- (`/Game/XC4VCharacter/XC4VCharacter.SiloMetalAmnt` (`self.XC4VCharacter`)) (`self.SiloSubtractoAmntSet`)) 0.025)
    (set `/Game/XC4VCharacter/XC4VCharacter.SiloMetalAmnt` (- (`/Game/XC4VCharacter/XC4VCharacter.SiloMetalAmnt` (`self.XC4VCharacter`)) (`self.SiloSubtractoAmntSet`)) (`self.XC4VCharacter`))
    (else
      (`self.SiloGameOver`))))

(event `SiloGameOver`
  (bind _metalsilo (`self.MetalSilo`))
  ;[1 1 1] SiloGameOver
  (`/Engine/EditorBlueprintResources/StandardMacros.DoOnce` false
    (:`Completed`
      (`|ExecutionSequence`
        (:`then_1`
          (`GameplayStatics.SpawnSound2D` "/Game/StarterContent/Audio/Explosion_Cue.Explosion_Cue" 0.8 1.0 0.0 null)
          (`AddComponent|NODE_AddParticleSystemComponent-0`)
          (`SceneComponent.SetVisibility` _metalsilo false false)
          (`SceneComponent.SetHiddenInGame` _metalsilo true false)
          (`self.DisableInput` (`self.XC4VCharacter`) (`GameplayStatics.GetPlayerController` 0))
          (goto _label_2 :!via `Open`))
        (:`then_2`
          (`GameplayStatics.SpawnSound2D` "/Game/Audio/AC/ShieldShuttingDown_Cue.ShieldShuttingDown_Cue" 1.0 1.0 0.0 null)
          (`KismetSystemLibrary.Delay` 3.0)
          (`/Engine/EditorBlueprintResources/StandardMacros.Gate` true :!label _label_2
            (:`Exit`
              (`|ExecutionSequence`
                (:`then_0`
                  (set `/Game/XC4VCharacter/XC4VCharacter.SiloMetalAmnt` 0.0 (`self.XC4VCharacter`)))
                (:`then_2`
                  ;;[1 1 1] Spawn GameOver Screen
                  (bind _returnvalue (`|CreateWidget` "/Game/Widgets/GameOverScreen.GameOverScreen_C"))
                  (`UserWidget.AddToViewport` _returnvalue 0))))))))))

(fn `UserConstructionScript`)