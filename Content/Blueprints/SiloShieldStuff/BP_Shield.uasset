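; Shield generator actor that tracks whether the player is sheltered and loses health while enemies overlap it.
; BeginPlay registers it on XC4VCharacter, which stores the shield health, and starts timelines used as update loops.
; These poll player and spawned-enemy overlaps, drain health, and destroy the shield with a sound at zero.
; Another loop animates the dynamic glass material between red and blue once waves start; ShieldRespawn is an empty stub.
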(event `self.ReceiveBeginPlay`
  ;[1 0 0] BeginPlay
  (`|ExecutionSequence`
    (:`then_0`
      ;[1 1 1] SavePlayer
      (bind _asxc4vcharacter (cast `/Game/XC4VCharacter/XC4VCharacter` (`GameplayStatics.GetPlayerCharacter` 0)))
      (set `self.XC4VCharacter` _asxc4vcharacter))
    (:`then_1`
      ;[1 1 1] Save Self as Shield
      (set `/Game/XC4VCharacter/XC4VCharacter.Shield` self (`self.XC4VCharacter`)))
    (:`then_2`
      ;[1 1 1] OverlapChecker
      (`self.CheckforOverlaps`))
    (:`then_3`
      (`self.ShieldRespawn`))
    (:`then_4`
      ;[1 1 1] ShieldHealthManagement
      (`|ExecutionSequence`
        (:`then_0`
          (`self.StatusChecking`))))
    (:`then_6`
      ;[1 1 1] WaveWarning
      (`self.WaveWarning`))
    (:`then_8`
      ;[1 1 1] Create Dynamic ShieldGlass Mat
      (bind _returnvalue (`PrimitiveComponent.CreateDynamicMaterialInstance` (`self.GeneratedShieldGlass`) 0 (`PrimitiveComponent.GetMaterial` (`self.GeneratedShieldGlass`) 0) "ShieldGlassDynMat"))
      (set `self.ShieldGlassDynMaterial` _returnvalue))))

(event `Shield Death`
  ;[1 1 1] Shield Life and Death
  (`/Engine/EditorBlueprintResources/StandardMacros.DoOnce` false :!label _label
    (:`Completed`
      (`GameplayStatics.SpawnSound2D` "/Game/Audio/AC/ShieldShuttingDown_Cue.ShieldShuttingDown_Cue" 1.0 1.0 0.0 null)
      (`|ExecutionSequence`
        (:`then_0`
          (set `/Game/XC4VCharacter/XC4VCharacter.ShieldAmnt` 0.0 (`self.XC4VCharacter`)))
        (:`then_1`
          (`self.K2_DestroyActor`))
        (:`then_2`
          (goto _label :!via `Reset`))))))

(event `ShieldRespawn`
  ;[1 1 1] Shield Life and Death
)

(event `ShieldReHealth`
  ;[1 1 1] Shield Life and Death
  (set `/Game/XC4VCharacter/XC4VCharacter.ShieldAmnt` 1000.0 (`self.XC4VCharacter`)))

(event `CheckforOverlaps`
  ;[1 1 1] OverlapChecker
  (`Timeline|CheckForOverlapsTimeline`
    (:`Update`
      (`|ExecutionSequence`
        (:`then_0`
          (if (`PrimitiveComponent.IsOverlappingActor` (`self.GeneratorColliderPlayer`) (`self.XC4VCharacter`))
            (set `self.isPlayerShielded?` true)
            (else
              (set `self.isPlayerShielded?` false))))
        (:`then_3`
          (for _array_element (`/Game/XC4VCharacter/XC4VCharacter.EnemiesSpawned` (`self.XC4VCharacter`)) :!label _label_2
            (`/Engine/EditorBlueprintResources/StandardMacros.IsValid` _array_element
              (:`Is Valid`
                (if (`PrimitiveComponent.IsOverlappingComponent` (`Character.CapsuleComponent` _array_element) (`self.GeneratorColliderEn`))
                  (set `self.isEnemyOverlapping?` true)
                  (else
                    (set `self.isEnemyOverlapping?` false))))))
          (`/Engine/EditorBlueprintResources/StandardMacros.DoOnce` false :!via `Reset`
            (:`Completed`
              (goto _label_2))))
        (:`then_4`
          (if (`self.isEnemyOverlapping?`)
            (`self.SubtractHealth` 2.0)))))))

(event `StatusChecking`
  ;[1 1 1] ShieldHealthManagement
  (`Timeline|StatusCheckingTimeline`
    (:`Update`
      (`|ExecutionSequence`
        (:`then_2`
          (if (<= (`/Game/XC4VCharacter/XC4VCharacter.ShieldAmnt` (`self.XC4VCharacter`)) 0.0)
            (`self.Shield Death`)))))))

(event `AddHealth`
  (params (ShieldHealthAmntAdjust :type "Float (double-precision)"))
  ;[1 1 1] ShieldHealthManagement
  (set `self.ShieldHealthAddAdjust` ShieldHealthAmntAdjust)
  (if (<= (+ (`/Game/XC4VCharacter/XC4VCharacter.ShieldAmnt` (`self.XC4VCharacter`)) (`self.ShieldHealthAddAdjust`)) 1000.0)
    (set `/Game/XC4VCharacter/XC4VCharacter.ShieldAmnt` (+ (`/Game/XC4VCharacter/XC4VCharacter.ShieldAmnt` (`self.XC4VCharacter`)) (`self.ShieldHealthAddAdjust`)) (`self.XC4VCharacter`))
    (else
      (`self.ShieldReHealth`))))

(event `SubtractHealth`
  (params (ShieldHealthSubtractAdjust :type "Float (double-precision)"))
  ;[1 1 1] ShieldHealthManagement
  (set `self.ShieldHealthSubtractAdjust` ShieldHealthSubtractAdjust)
  (if (>= (- (`/Game/XC4VCharacter/XC4VCharacter.ShieldAmnt` (`self.XC4VCharacter`)) (`self.ShieldHealthSubtractAdjust`)) 0.0)
    (set `/Game/XC4VCharacter/XC4VCharacter.ShieldAmnt` (- (`/Game/XC4VCharacter/XC4VCharacter.ShieldAmnt` (`self.XC4VCharacter`)) (`self.ShieldHealthSubtractAdjust`)) (`self.XC4VCharacter`))
    (else
      (set `/Game/XC4VCharacter/XC4VCharacter.ShieldAmnt` 0.0 (`self.XC4VCharacter`))
      (`self.Shield Death`))))

(event `WaveWarning`
  (bind (_glassred_r _glassred_g _glassred_b) (break `LinearColor` (`self.GlassRed`)))
  (bind (_glassblue_r _glassblue_g _glassblue_b) (break `LinearColor` (`self.GlassBlue`)))
  ;[1 1 1] WaveWarning
  (`Timeline|WaveWarningTimeline`
    (:`Update`
      (if (`/Game/XC4VCharacter/XC4VCharacter.isWavesStarted?` (`self.XC4VCharacter`))
        (bind (_direction _glasswarningtimelinecurve) (`Timeline|GlassWarningTimeline`)
          (:`Update`
            (`|ExecutionSequence`
              (:`then_0`
                (bind (_returnvalue_x _returnvalue_y _returnvalue_z) (`KismetMathLibrary.BreakVector` (`KismetMathLibrary.VLerp` (`KismetMathLibrary.MakeVector` _glassred_r _glassred_g _glassred_b) (`KismetMathLibrary.MakeVector` _glassblue_r _glassblue_g _glassblue_b) _glasswarningtimelinecurve)))
                (`MaterialInstanceDynamic.SetVectorParameterValue` (`self.ShieldGlassDynMaterial`) "ColorGlass" (make `LinearColor` _returnvalue_x _returnvalue_y _returnvalue_z 1.0))))))
        (else
          (`MaterialInstanceDynamic.SetVectorParameterValue` (`self.ShieldGlassDynMaterial`) "ColorGlass" (`self.GlassBlue`)))))))

(fn `UserConstructionScript`)