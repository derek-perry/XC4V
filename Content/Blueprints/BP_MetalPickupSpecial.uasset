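; Special metal pickup that the player collects by overlapping it while drilling, granting metal and special status.
; A timeline started at BeginPlay polls for overlap with the cached XC4V character and triggers a one-time pickup.
; A second timeline sweeps the metal ball toward the drill using a curve-driven lerp.
; When it finishes, it sets IsSpecial, adds metal up to a cap, shows a HUD message and destroys itself.
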(event `self.ReceiveBeginPlay`
  ;[1 1 1] Begin Play
  (`|ExecutionSequence`
    (:`then_0`
      ;[1 1 1] Save Character
      (bind _asxc4vcharacter (cast `/Game/XC4VCharacter/XC4VCharacter` (`GameplayStatics.GetPlayerCharacter` 0)))
      (set `self.XC4VCharacter` _asxc4vcharacter))
    (:`then_1`
      ;[1 1 1] Call Events
      (`self.PickupCheckforPlayer`))))

(event `PickupCheckforPlayer`
  ;[1 1 1] If Player Overlap, do Pickup
  (`Timeline|PCheck4Player`
    (:`Update`
      (if (`self.IsOverlappingActor` (`self.XC4VCharacter`))
        (if (`/Game/XC4VCharacter/XC4VCharacter.isDrilling?` (`self.XC4VCharacter`))
          (`self.InitPickup`))))))

(event `InitPickup`
  ;[1 1 1] Do The Picking Up
  (`/Engine/EditorBlueprintResources/StandardMacros.DoOnce` false
    (:`Completed`
      (`|ExecutionSequence`
        (:`then_0`
          ;;[1 1 1] MetalPickup Move to Player's Drill
          (bind (_direction _metalpickuptimelinecurve) (`Timeline|MetalPickupTimeline`)
            (:`Update`
              (`SceneComponent.K2_SetWorldLocation` (`self.MetalBall`) (`KismetMathLibrary.VLerp` (`SceneComponent.K2_GetComponentLocation` (`/Game/XC4VCharacter/XC4VCharacter.BP_XC4VDrill` (`self.XC4VCharacter`))) (`SceneComponent.K2_GetComponentLocation` (`self.MetalBall`)) _metalpickuptimelinecurve) true false))
            (:`Finished`
              (`|ExecutionSequence`
                (:`then_0`
                  ;;[1 1 1] Check if Still Special
                  (if (not (`/Game/XC4VCharacter/XC4VCharacter.isSpecial?` (`self.XC4VCharacter`)))
                    (set `/Game/XC4VCharacter/XC4VCharacter.isSpecial?` true (`self.XC4VCharacter`))))
                (:`then_1`
                  ;;[1 1 1] Adjust Metal Amount
                  (if (< (`/Game/XC4VCharacter/XC4VCharacter.MetalAmount` (`self.XC4VCharacter`)) (- 100.0 (`self.SpecialMetalPickupAmount`)))
                    (set `/Game/XC4VCharacter/XC4VCharacter.MetalAmount` (+ (`/Game/XC4VCharacter/XC4VCharacter.MetalAmount` (`self.XC4VCharacter`)) (`self.SpecialMetalPickupAmount`)) (`self.XC4VCharacter`))
                    (`/Game/Widgets/W_Info.DebugMessage` (`/Game/XC4VCharacter/XC4VCharacter.HUDInfo` (`self.XC4VCharacter`)) "+45 SPECIAL Metal added to Cannon!" (struct :`G` 1.0 :`A` 1.0))
                    (else
                      (set `/Game/XC4VCharacter/XC4VCharacter.MetalAmount` 100.0 (`self.XC4VCharacter`))
                      (`/Game/Widgets/W_Info.DebugMessage` (`/Game/XC4VCharacter/XC4VCharacter.HUDInfo` (`self.XC4VCharacter`)) "You collected a SPECIAL METAL!" (struct :`R` 1.0 :`B` 0.796064 :`A` 1.0)))))
                (:`then_2`
                  (`self.K2_DestroyActor`))))))))))

(fn `UserConstructionScript`)