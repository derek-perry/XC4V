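; BP_Comm is a proximity message point that shows a floating BP_CommText while the player is inside its CommMessageArea.
; Two timelines started on BeginPlay act as update loops: one polls overlap to set IsPlayerClose, the other drives the display from that flag.
; A DoOnce spawns the text at MessageSpawnPoint, which then turns toward the first-person camera with a pitch offset.
; Leaving the area destroys the text and resets the gate.
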(event `self.ReceiveBeginPlay`
  ;[1 0 0] BeginPlay
  (`|ExecutionSequence`
    (:`then_0`
      ;[1 1 1] SavePlayer
      (bind _asxc4vcharacter (cast `/Game/XC4VCharacter/XC4VCharacter` (`GameplayStatics.GetPlayerCharacter` 0)))
      (set `self.XC4VCharacter` _asxc4vcharacter))
    (:`then_1`
      ;[1 1 1] BeginCheckingforPlayer
      (`self.CheckforPlayer`))
    (:`then_2`
      ;[1 1 1] Start Timeline For Message Displaying
      (`self.DisplayMessage`))))

(event `CheckforPlayer`
  ;[1 1 1] CheckPlayerOverlap set isPlayerClose if or ifnot
  (`Timeline|PlayerCheckTimeline`
    (:`Update`
      (if (`PrimitiveComponent.IsOverlappingActor` (`self.CommMessageArea`) (`self.XC4VCharacter`))
        (set `self.isPlayerClose?` true)
        (else
          (set `self.isPlayerClose?` false))))))

(event `DisplayMessage`
  (bind _commtextspawned (`self.CommTextSpawned`))
  (bind (_returnvalue_roll _returnvalue_pitch _returnvalue_yaw) (`KismetMathLibrary.BreakRotator` (`KismetMathLibrary.FindLookAtRotation` (`SceneComponent.K2_GetComponentLocation` (`self.MessageSpawnPoint`)) (`SceneComponent.K2_GetComponentLocation` (`/Game/AdvancedLocomotionV3/Blueprints/ALS_BaseCharacter.FP_Camera` (`self.XC4VCharacter`))))))
  ;[1 1 1] DisplayMessage when Player is Close
  (`Timeline|DisplayMessageTimeline`
    (:`Update`
      (if (`self.isPlayerClose?`)
        (`|ExecutionSequence`
          (:`then_0`
            ;;[1 1 1] When player is close, Spawn CommMessage and Set Text
            (`/Engine/EditorBlueprintResources/StandardMacros.DoOnce` false :!label _label
              (:`Completed`
                (bind _returnvalue (`|SpawnActorFromClass` "/Game/Blueprints/BP_CommText.BP_CommText_C" (`SceneComponent.K2_GetComponentToWorld` (`self.MessageSpawnPoint`)) "AlwaysSpawn" "OverrideRootScale" null null))
                (set `self.CommTextSpawned` _returnvalue)
                (set `/Game/Blueprints/BP_CommText.CommText` (`self.CommText`) (`self.CommTextSpawned`)))))
          (:`then_1`
            ;;[1 1 1] SetRotation towards Player
            (if (`KismetSystemLibrary.IsValid` (`self.CommTextSpawned`))
              (set `self.CommRotationOld` (`self.CommRotation`))
              (set `self.CommRotation` (`KismetMathLibrary.MakeRotator` _returnvalue_roll (+ _returnvalue_pitch 20.0) _returnvalue_yaw))
              (`self.K2_SetActorRotation` (`self.CommTextSpawned`) (`KismetMathLibrary.RInterpTo` (`self.CommRotationOld`) (`self.CommRotation`) (`GameplayStatics.GetWorldDeltaSeconds`) 0.1) false))))
        (else
          ;;[1 1 1] Else Delete Comm Message
          (if (`KismetSystemLibrary.IsValid` _commtextspawned)
            (`self.K2_DestroyActor` _commtextspawned)
            (goto _label :!via `Reset`)
            (else
              (goto _label :!via `Reset`))))))))

(fn `UserConstructionScript`)