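; Enemy turret that turns toward the player when PawnSensing sees them and fires projectiles on a cooldown.
; Spray or slug impacts freeze it temporarily, halting aim and fire; hammer hits damage it, or kill it outright while frozen.
; Timelines serve as update loops for player proximity, hammer overlap, zero-health death and state-based material swaps (frozen, hurt, dying, alert, idle).
; Death posts a HUD message, adds a particle component and destroys the actor.
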(event `self.ReceiveBeginPlay`
  ;[1 1 1] Begin Play
  ;[1 1 1] SaveEnemySpawnPoint
  (set `self.EnemySpawnPoint` (`self.GetTransform`))
  ;[1 1 1] Save Player
  (bind _asxc4vcharacter (cast `/Game/XC4VCharacter/XC4VCharacter` (`GameplayStatics.GetPlayerCharacter` 0)))
  (set `self.XC4VCharacter` _asxc4vcharacter)
  ;[1 1 1] Start Checking for Player
  (`self.CheckPlayerNearEnemy`)
  ;[1 1 1] Init HammerHitChecker
  (`self.HammerHitCheck`)
  ;[1 1 1] Init EnemyCheck
  (`self.EnemyCheck`))

(event `self.PawnSensing.OnSeePawn`
  (params (Pawn :type "Pawn Object Reference"))
  ;[1 1 1] On Sense Player, Follow Player
  (cast `/Game/XC4VCharacter/XC4VCharacter` Pawn
    (:`then`
      (set `self.isEnemying?` true)
      (if (not (`self.isFrozen?`))
        (`|ExecutionSequence`
          (:`then_0`
            ;;[1 1 1] Rotate Toward Player
            (bind _output_get (set `self.EnemyToPlayerRot` (`KismetMathLibrary.FindLookAtRotation` (`SceneComponent.K2_GetComponentLocation` (`self.Enemy`)) (`SceneComponent.K2_GetComponentLocation` (`Actor.RootComponent` (`self.XC4VCharacter`))))))
            (`self.K2_SetActorRotation` _output_get))
          (:`then_1`
            ;;[1 1 1] Fire Projectile
            (if (`self.canProjectile?`)
              (`|SpawnActorFromClass` "/Game/Blueprints/BP_EnemyProjectile.BP_EnemyProjectile_C" (`KismetMathLibrary.MakeTransform` (`SceneComponent.K2_GetComponentLocation` (`self.ProjectileSpawn`)) (`self.EnemyToPlayerRot`)) "Undefined" "OverrideRootScale" null null)
              (set `self.canProjectile?` false)
              (`KismetSystemLibrary.RetriggerableDelay` (`self.ProjectileDelay`))
              (set `self.canProjectile?` true))))))
    (:`CastFailed`
      (set `self.isEnemying?` false))))

(event `self.HitImpactRadius.OnComponentBeginOverlap`
  (params (OverlappedComponent :type "PrimitiveComponent Object Reference") (OtherActor :type "Actor Object Reference") (OtherComp :type "PrimitiveComponent Object Reference") (OtherBodyIndex :type Integer) (bFromSweep :type Boolean) (SweepResult :type "HitResult Structure (by ref)"))
  ;[1 1 1] OnSprayHit
  (cast `/Game/Blueprints/BP_SprayImpact` OtherActor)
  (if (not (`self.isFrozen?`))
    (`|ExecutionSequence`
      (:`then_0`
        (set `self.isFrozen?` true)
        (`PrimitiveComponent.SetMaterial` (`self.Enemy`) 0 (`self.FrozenMaterial`)))
      (:`then_3`
        (`KismetSystemLibrary.RetriggerableDelay` (`self.FrozenTime`))
        (if (`self.isFrozen?`)
          (set `self.isFrozen?` false)
          (`|ExecutionSequence`
            (:`then_1`
              ;[1 1 1] Check for Enemy States and update Enemy
              ;;[1 1 1] Active/Enemying
              (if (`self.isEnemying?`) :!label _label
                ;;[1 1 1] Frozen
                (if (`self.isFrozen?`)
                  (`PrimitiveComponent.SetMaterial` (`self.Enemy`) 0 (`self.FrozenMaterial`))
                  (else
                    ;;[1 1 1] Injury/Ouch
                    (if (`self.isOuch?`)
                      (`PrimitiveComponent.SetMaterial` (`self.Enemy`) 0 (`self.OuchMaterial`))
                      (else
                        ;;[1 1 1] Dieing
                        (if (`self.isDieing?`)
                          (`PrimitiveComponent.SetMaterial` (`self.Enemy`) 0 (`self.DieMaterial`))
                          (else
                            (`PrimitiveComponent.SetMaterial` (`self.Enemy`) 0 (`self.EnemyMaterial`))))))))
                (else
                  ;;[1 1 1] Frozen
                  (if (`self.isFrozen?`)
                    (`PrimitiveComponent.SetMaterial` (`self.Enemy`) 0 (`self.FrozenMaterial`))
                    (else
                      ;;[1 1 1] Injury/Ouch
                      (if (`self.isOuch?`)
                        (`PrimitiveComponent.SetMaterial` (`self.Enemy`) 0 (`self.OuchMaterial`))
                        (else
                          ;;[1 1 1] Dieing
                          (if (`self.isDieing?`)
                            (`PrimitiveComponent.SetMaterial` (`self.Enemy`) 0 (`self.DieMaterial`))
                            (else
                              ;;[1 1 1] Else Grey
                              (`PrimitiveComponent.SetMaterial` (`self.Enemy`) 0 (`self.GreyMaterial`)))))))))))))))))

(event `self.SlugImpactRadius.OnComponentBeginOverlap`
  (params (OverlappedComponent :type "PrimitiveComponent Object Reference") (OtherActor :type "Actor Object Reference") (OtherComp :type "PrimitiveComponent Object Reference") (OtherBodyIndex :type Integer) (bFromSweep :type Boolean) (SweepResult :type "HitResult Structure (by ref)"))
  ;[1 1 1] OnSlugHit
  (cast `/Game/Blueprints/BP_SlugImpact` OtherActor)
  (if (not (`self.isFrozen?`))
    (`|ExecutionSequence`
      (:`then_0`
        (set `self.isFrozen?` true)
        (`PrimitiveComponent.SetMaterial` (`self.Enemy`) 0 (`self.FrozenMaterial`)))
      (:`then_3`
        (`KismetSystemLibrary.RetriggerableDelay` (`self.FrozenTime`))
        (if (`self.isFrozen?`)
          (set `self.isFrozen?` false)
          (`|ExecutionSequence`
            (:`then_1`
              (goto _label))))))))

(event `HammerHitCheck`
  ;[1 1 1] Check if player is Hammerhitting
  (`Timeline|HammerHitChecker`
    (:`Update`
      (if (and (`PrimitiveComponent.IsOverlappingComponent` (`self.HitImpactRadius`) (`/Game/XC4VCharacter/XC4VCharacter.HitCollider` (`self.XC4VCharacter`))) (`/Game/XC4VCharacter/XC4VCharacter.isHammering?` (`self.XC4VCharacter`)))
        (if (`self.isFrozen?`)
          (`self.DIEZOMBIE`)
          (else
            (`self.OUCHZOMBIE`)))))))

(event `OUCHZOMBIE`
  ;[1 1 1] Bot Injury
  (if (not (`self.isOuch?`))
    (set `self.isOuch?` true)
    (`|ExecutionSequence`
      (:`then_0`
        (`PrimitiveComponent.SetMaterial` (`self.Enemy`) 0 (`self.OuchMaterial`)))
      (:`then_1`
        (`KismetSystemLibrary.RetriggerableDelay` 0.1)
        (`|ExecutionSequence`
          (:`then_0`
            (set `self.isOuch?` false))
          (:`then_1`
            (goto _label))))
      (:`then_2`
        (set `self.BotHealth` (- (`self.BotHealth`) 6.9))))))

(event `DIEZOMBIE`
  ;[1 1 1] Bot Death
  (if (not (`self.isDieing?`))
    (set `self.isDieing?` true)
    (`PrimitiveComponent.SetMaterial` (`self.Enemy`) 0 (`self.DieMaterial`))
    ;;[1 1 1] Send Message About An Enemy being Killed
    (bind _asxc4vcharacter (cast `/Game/XC4VCharacter/XC4VCharacter` (`GameplayStatics.GetPlayerCharacter` 0)))
    (`/Game/Widgets/W_Info.DebugMessage` (`/Game/XC4VCharacter/XC4VCharacter.HUDInfo` _asxc4vcharacter) "BOT ELIMINATED!" (struct :`R` 1.0 :`G` 0.111022 :`A` 1.0))
    (bind _returnvalue (`AddComponent|NODE_AddParticleSystemComponent-1` :`RelativeTransform` (`KismetMathLibrary.MakeTransform` (`SceneComponent.RelativeLocation` (`self.Mesh`)))))
    (set `self.ExplosionParticles` _returnvalue)
    (`self.K2_DestroyActor`)))

(event `EnemyCheck`
  ;[1 1 1] Check for Enemy States and update Enemy
  (`Timeline|EnemyCheckTimeline`
    (:`Update`
      (`|ExecutionSequence`
        (:`then_1`
          (goto _label))
        (:`then_2`
          ;;[1 1 1] Health Death
          (if (< (`self.BotHealth`) 0.0)
            (`self.DIEZOMBIE`)))))))

(event `CheckPlayerNearEnemy`
  ;[1 1 1] Check if Player is Near Enemy
  (`Timeline|EnemyPlayerChecker`
    (:`Update`
      (if (`PrimitiveComponent.IsOverlappingActor` (`self.EnemyInteractRadius`) (`self.XC4VCharacter`))
        (set `self.isEnemying?` true)
        (else
          (set `self.isEnemying?` false))))))

(fn `UserConstructionScript`)