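; BP_Silo is a silo that displays the player character's metal amount as a lava level on its mesh.
; On BeginPlay it registers itself on the XC4VCharacter player and swaps the MetalSilo mesh's first material for a dynamic instance.
; A timeline then acts as an updater, reading the character's MetalAmount and writing its inverse (one minus the value) to the LavaLevelAmnt material parameter.
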(event `self.ReceiveBeginPlay`
  (bind _silolavamaterial (`self.SiloLavaMaterial`))
  (`|ExecutionSequence`
    (:`then_0`
      ;[1 1 1] SavePlayer and silo
      (bind _asxc4vcharacter (cast `/Game/XC4VCharacter/XC4VCharacter` (`GameplayStatics.GetPlayerCharacter` 0)))
      (set `self.XC4VCharacter` _asxc4vcharacter)
      (set `/Game/XC4VCharacter/XC4VCharacter.Silo` self (`self.XC4VCharacter`)))
    (:`then_1`
      ;[1 1 1] Get and Set Material for Lava amount
      (set `self.SiloLavaMaterial` (`PrimitiveComponent.GetMaterial` (`self.MetalSilo`) 0))
      (bind _returnvalue (`KismetMaterialLibrary.CreateDynamicMaterialInstance` _silolavamaterial _silolavamaterial "DynSiloLavaMat"))
      (set `self.DynamicSiloLavaMat` _returnvalue)
      (`PrimitiveComponent.SetMaterial` (`self.MetalSilo`) 0 (`self.DynamicSiloLavaMat`)))
    (:`then_2`
      ;[1 1 1] Start Setting Laval Level
      (`self.SetLavaAmnt`))))

(event `SetLavaAmnt`
  ;[1 1 1] Set Lava Level Display
  (`Timeline|SetLavaAmntTimeline`
    (:`Update`
      ;;[1 1 1] Lava amnt
      (bind _output_get (set `self.SiloLavaLevelAmnt` (`/Game/XC4VCharacter/XC4VCharacter.MetalAmount` (`self.XC4VCharacter`))))
      (`MaterialInstanceDynamic.SetScalarParameterValue` (`self.DynamicSiloLavaMat`) "LavaLevelAmnt" (- 1.0 _output_get)))))

(fn `UserConstructionScript`)