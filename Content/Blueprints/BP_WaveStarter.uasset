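; Wave trigger actor that starts an enemy wave the first time the player character overlaps it.
; It posts a HUD debug message, then after a short delay plays a timeline whose updates drive a randomly limited DoN.
; That spawns silo attackers at random offsets around component A.
; Limit, completion check and reported count each roll separate random numbers, so the announced total can differ from the actual spawns.
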(event `self.ReceiveBeginPlay`
  ;[1 1 1] BeginPlay
  (`|ExecutionSequence`
    (:`then_0`
      ;[1 1 1] SavePlayer
      (bind _asxc4vcharacter (cast `/Game/XC4VCharacter/XC4VCharacter` (`GameplayStatics.GetPlayerCharacter` 0)))
      (set `self.XC4VCharacter` _asxc4vcharacter))))

(event `self.ReceiveActorBeginOverlap`
  (params (OtherActor :type "Actor Object Reference"))
  ;[1 1 1] On Overlap, Teleport
  (cast `/Game/XC4VCharacter/XC4VCharacter` OtherActor)
  ;[1 1 1] Send Message
  (`/Engine/EditorBlueprintResources/StandardMacros.DoOnce` false
    (:`Completed`
      (`/Game/Widgets/W_Info.DebugMessage` (`/Game/XC4VCharacter/XC4VCharacter.HUDInfo` (`self.XC4VCharacter`)) "Wave Started!" (struct :`R` 1.0 :`B` 0.018721 :`A` 1.0))
      (`KismetSystemLibrary.RetriggerableDelay` 1.0)
      ;[1 1 1] Start Wave A
      (`self.WaveA`))))

(event `WaveA`
  (bind _returnvalue (`KismetMathLibrary.RandomFloatInRange` -200.0 200.0))
  (bind (_returnvalue_x _returnvalue_y _returnvalue_z) (`KismetMathLibrary.BreakVector` (`SceneComponent.K2_GetComponentLocation` (`self.A`))))
  (bind _returnvalue_2 (`KismetMathLibrary.FTrunc` (`KismetMathLibrary.RandomFloatInRange` 4.0 10.0)))
  ;[1 1 1] Spawn Enemies
  (`Timeline|WaveATimeline`
    (:`Update`
      (bind _counter (`/Engine/EditorBlueprintResources/StandardMacros.Do N` _returnvalue_2)
        (:`Exit`
          (if (>= _counter _returnvalue_2)
            (`/Game/Widgets/W_Info.DebugMessage` (`/Game/XC4VCharacter/XC4VCharacter.HUDInfo` (`self.XC4VCharacter`)) (`KismetTextLibrary.Conv_StringToText` (`KismetStringLibrary.Concat_StrStr` (`KismetStringLibrary.Conv_IntToString` _returnvalue_2) " Enemies Spawned!")) (struct :`R` 1.0 :`B` 0.018721 :`A` 1.0))
            (else
              (`|SpawnActorFromClass` "/Game/Blueprints/BP_EnemySiloAttacker.BP_EnemySiloAttacker_C" (`KismetMathLibrary.MakeTransform` (`KismetMathLibrary.MakeVector` (+ _returnvalue_x _returnvalue) (+ _returnvalue_y _returnvalue) (+ _returnvalue_z _returnvalue)) (struct)) "AlwaysSpawn" "OverrideRootScale" null null))))))))

(fn `UserConstructionScript`)