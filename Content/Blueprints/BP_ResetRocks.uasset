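; Trigger actor that resets a field of destructible-style rock pickups or obstacles when the player character overlaps it.
; BeginPlay spawns the initial rocks through SpawnRocks, which places a hard-coded 3x3 grid and stores references, though the third slot has no class set.
; An XC4VCharacter overlap destroys all actors of four rock classes, respawns the grid and shows a "Rocks Reset!" HUD message.
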(event `self.ReceiveBeginPlay`
  ;[1 1 1] Spawn Rocks at first
  (`/Engine/EditorBlueprintResources/StandardMacros.DoOnce` false
    (:`Completed`
      (`self.Spawn Rocks`))))

(event `Spawn Rocks`
  ;[1 1 1] Spawn New Rocks
  (bind _returnvalue (`|SpawnActorFromClass` "/Game/Blueprints/BP_StandardRock.BP_StandardRock_C" (`KismetMathLibrary.MakeTransform` (1450.0 -478.0 25.0)) "Undefined" "OverrideRootScale" null null))
  (set `self.Rock1` _returnvalue)
  (bind _returnvalue_2 (`|SpawnActorFromClass` "/Game/Blueprints/BP_StandardRock.BP_StandardRock_C" (`KismetMathLibrary.MakeTransform` (1450.0 4.706848 25.0)) "Undefined" "OverrideRootScale" null null))
  (set `self.Rock2` _returnvalue_2)
  (`|SpawnActorFromClass` "/Game/Blueprints/BP_SpecialRock.BP_SpecialRock_C" (`KismetMathLibrary.MakeTransform` (1450.0 450.827637 25.0) (struct)) "Undefined" "OverrideRootScale" null null)
  (set `self.Rock3` null)
  (bind _returnvalue_3 (`|SpawnActorFromClass` "/Game/Blueprints/BP_StandardRock.BP_StandardRock_C" (`KismetMathLibrary.MakeTransform` (2031.74231 -478.0 25.0)) "Undefined" "OverrideRootScale" null null))
  (set `self.Rock4` _returnvalue_3)
  (bind _returnvalue_4 (`|SpawnActorFromClass` "/Game/Blueprints/BP_StandardRock.BP_StandardRock_C" (`KismetMathLibrary.MakeTransform` (2031.74231 4.706848 25.0)) "Undefined" "OverrideRootScale" null null))
  (set `self.Rock5` _returnvalue_4)
  (bind _returnvalue_5 (`|SpawnActorFromClass` "/Game/Blueprints/BP_StandardRock.BP_StandardRock_C" (`KismetMathLibrary.MakeTransform` (2031.74231 450.827637 25.0)) "Undefined" "OverrideRootScale" null null))
  (set `self.Rock6` _returnvalue_5)
  (bind _returnvalue_6 (`|SpawnActorFromClass` "/Game/Blueprints/BP_StandardRock.BP_StandardRock_C" (`KismetMathLibrary.MakeTransform` (2751.272461 -478.0 25.0)) "Undefined" "OverrideRootScale" null null))
  (set `self.Rock7` _returnvalue_6)
  (bind _returnvalue_7 (`|SpawnActorFromClass` "/Game/Blueprints/BP_StandardRock.BP_StandardRock_C" (`KismetMathLibrary.MakeTransform` (2751.272461 4.706848 25.0)) "Undefined" "OverrideRootScale" null null))
  (set `self.Rock8` _returnvalue_7)
  (bind _returnvalue_8 (`|SpawnActorFromClass` "/Game/Blueprints/BP_StandardRock.BP_StandardRock_C" (`KismetMathLibrary.MakeTransform` (2751.272461 450.827637 25.0)) "Undefined" "OverrideRootScale" null null))
  (set `self.Rock9` _returnvalue_8))

(event `self.ReceiveActorBeginOverlap`
  (params (OtherActor :type "Actor Object Reference"))
  ;[1 1 1] If Player overlaps rock reseter, Destroy old rocks and call for new rocks
  (cast `/Game/XC4VCharacter/XC4VCharacter` OtherActor)
  (`|ExecutionSequence`
    (:`then_0`
      (bind _outactors (`GameplayStatics.GetAllActorsOfClass` "/Game/Blueprints/BP_DRock.BP_DRock_C"))
      (`self.K2_DestroyActor` _outactors))
    (:`then_1`
      (bind _outactors_2 (`GameplayStatics.GetAllActorsOfClass` "/Game/Blueprints/BP_DRockSpecial.BP_DRockSpecial_C"))
      (`self.K2_DestroyActor` _outactors_2))
    (:`then_2`
      (bind _outactors_3 (`GameplayStatics.GetAllActorsOfClass` "/Game/Blueprints/BP_StandardRock.BP_StandardRock_C"))
      (`self.K2_DestroyActor` _outactors_3))
    (:`then_3`
      (bind _outactors_4 (`GameplayStatics.GetAllActorsOfClass` "/Game/Blueprints/BP_SpecialRock.BP_SpecialRock_C"))
      (`self.K2_DestroyActor` _outactors_4))
    (:`then_4`
      (`self.Spawn Rocks`))
    (:`then_5`
      (bind _asxc4vcharacter (cast `/Game/XC4VCharacter/XC4VCharacter` (`GameplayStatics.GetPlayerCharacter` 0)))
      (`/Game/HUD/W_Info.ScreenMessage` (`/Game/XC4VCharacter/XC4VCharacter.HUDInfo` _asxc4vcharacter) "Rocks Reset!" (struct :`G` 0.5 :`B` 1.0 :`A` 1.0)))))

(fn `UserConstructionScript`)