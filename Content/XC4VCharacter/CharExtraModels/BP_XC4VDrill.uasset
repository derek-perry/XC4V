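; BP_XC4VDrill is the XC4V character's drill actor, which kills bot zombies it strikes.
; On BeginPlay it caches the player's XC4V character and that character's Bot1 and Bot2 references.
; When its collider hits either bot while the character is drilling or hammering, it calls DIEZOMBIE on that bot.
; Hits on any other actor only print a debug string.
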(event `self.ReceiveBeginPlay`
  (bind _asxc4vcharacter (cast `/Game/XC4VCharacter/XC4VCharacter` (`GameplayStatics.GetPlayerCharacter` 0)))
  (set `self.XC4VCharacter` _asxc4vcharacter)
  (set `self.Bot1` (`/Game/XC4VCharacter/XC4VCharacter.Bot1` _asxc4vcharacter))
  (set `self.Bot2` (`/Game/XC4VCharacter/XC4VCharacter.Bot2` _asxc4vcharacter)))

(event `self.xc4vdrillcollider.OnComponentHit`
  (params (HitComponent :type "PrimitiveComponent Object Reference") (OtherActor :type "Actor Object Reference") (OtherComp :type "PrimitiveComponent Object Reference") (NormalImpulse :type "Vector Structure") (Hit :type "HitResult Structure (by ref)"))
  (bind _bot1 (`self.Bot1`))
  (bind _bot2 (`self.Bot2`))
  (bind _xc4vcharacter (`self.XC4VCharacter`))
  (bind _xc4vcharacter_2 (`self.XC4VCharacter`))
  (if (== OtherActor _bot1)
    (if (or (`/Game/XC4VCharacter/XC4VCharacter.isDrilling?` _xc4vcharacter_2) (`/Game/XC4VCharacter/XC4VCharacter.isHammering?` _xc4vcharacter_2))
      (`/Game/AdvancedLocomotionV3/Blueprints/MannequinCharacter.DIEZOMBIE` _bot1))
    (elif (== OtherActor _bot2)
      (if (or (`/Game/XC4VCharacter/XC4VCharacter.isDrilling?` _xc4vcharacter) (`/Game/XC4VCharacter/XC4VCharacter.isHammering?` _xc4vcharacter))
        (`/Game/AdvancedLocomotionV3/Blueprints/MannequinCharacter.DIEZOMBIE` _bot2))
      (else
        (`KismetSystemLibrary.PrintString` "What Happened?")))))

(fn `UserConstructionScript`)