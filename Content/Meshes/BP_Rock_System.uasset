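; Rock field manager that spawns a grid of nine BP_StandardRock actors and resets it when an actor overlaps it.
; SpawnRocks, called on BeginPlay, places the rocks at hard-coded transforms in three rows of three and stores each reference.
; Any overlap destroys every BP_DRock and BP_StandardRock found through GetAllActorsOfClass, then calls SpawnRocks again for a fresh layout.
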(event `Spawn Rocks`
  (bind _returnvalue (`|SpawnActorFromClass` "/Game/Blueprints/BP_StandardRock.BP_StandardRock_C" (`KismetMathLibrary.MakeTransform` (1450.0 -478.0 0.0)) "Undefined" "OverrideRootScale" null null))
  (set `self.Rock1` _returnvalue)
  (bind _returnvalue_2 (`|SpawnActorFromClass` "/Game/Blueprints/BP_StandardRock.BP_StandardRock_C" (`KismetMathLibrary.MakeTransform` (1450.0 4.706848 0.0)) "Undefined" "OverrideRootScale" null null))
  (set `self.Rock2` _returnvalue_2)
  (bind _returnvalue_3 (`|SpawnActorFromClass` "/Game/Blueprints/BP_StandardRock.BP_StandardRock_C" (`KismetMathLibrary.MakeTransform` (1450.0 450.827637 0.0)) "Undefined" "OverrideRootScale" null null))
  (set `self.Rock3` _returnvalue_3)
  (bind _returnvalue_4 (`|SpawnActorFromClass` "/Game/Blueprints/BP_StandardRock.BP_StandardRock_C" (`KismetMathLibrary.MakeTransform` (2031.74231 -478.0 0.0)) "Undefined" "OverrideRootScale" null null))
  (set `self.Rock4` _returnvalue_4)
  (bind _returnvalue_5 (`|SpawnActorFromClass` "/Game/Blueprints/BP_StandardRock.BP_StandardRock_C" (`KismetMathLibrary.MakeTransform` (2031.74231 4.706848 0.0)) "Undefined" "OverrideRootScale" null null))
  (set `self.Rock5` _returnvalue_5)
  (bind _returnvalue_6 (`|SpawnActorFromClass` "/Game/Blueprints/BP_StandardRock.BP_StandardRock_C" (`KismetMathLibrary.MakeTransform` (2031.74231 450.827637 0.0)) "Undefined" "OverrideRootScale" null null))
  (set `self.Rock6` _returnvalue_6)
  (bind _returnvalue_7 (`|SpawnActorFromClass` "/Game/Blueprints/BP_StandardRock.BP_StandardRock_C" (`KismetMathLibrary.MakeTransform` (2751.272461 -478.0 0.0)) "Undefined" "OverrideRootScale" null null))
  (set `self.Rock7` _returnvalue_7)
  (bind _returnvalue_8 (`|SpawnActorFromClass` "/Game/Blueprints/BP_StandardRock.BP_StandardRock_C" (`KismetMathLibrary.MakeTransform` (2751.272461 4.706848 0.0)) "Undefined" "OverrideRootScale" null null))
  (set `self.Rock8` _returnvalue_8)
  (bind _returnvalue_9 (`|SpawnActorFromClass` "/Game/Blueprints/BP_StandardRock.BP_StandardRock_C" (`KismetMathLibrary.MakeTransform` (2751.272461 450.827637 0.0)) "Undefined" "OverrideRootScale" null null))
  (set `self.Rock9` _returnvalue_9))

(event `self.ReceiveBeginPlay`
  (`self.Spawn Rocks`))

(event `self.ReceiveActorBeginOverlap`
  (params (OtherActor :type "Actor Object Reference"))
  (bind _outactors (`GameplayStatics.GetAllActorsOfClass` "/Game/Blueprints/BP_DRock.BP_DRock_C"))
  (`self.K2_DestroyActor` _outactors)
  (bind _outactors_2 (`GameplayStatics.GetAllActorsOfClass` "/Game/Blueprints/BP_StandardRock.BP_StandardRock_C"))
  (`self.K2_DestroyActor` _outactors_2)
  (`self.Spawn Rocks`))

(fn `UserConstructionScript`)